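; Tutorial-map player camera for a Brexit border-control game about checking travelers and packages, showing the tutorial widget on start.
; Clicks trace under the cursor to ClickedEvent actors; helpers spawn document grids from traveler or package flags and slide in description panels.
; Timelines drain human and package gauges, adjusted by right or wrong calls and difficulty.
; Also holds the day clock ending in BrexitMap, data-table daily news and save/load.
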(fn `DestroyPaperHuman`
  (bind _tabofpaperhuman (`self.TabOfPaperHuman`))
  (for _array_element _tabofpaperhuman
    (`self.K2_DestroyActor` _array_element))
  (`KismetArrayLibrary.Array_Clear` _tabofpaperhuman)
  (`KismetArrayLibrary.Array_Clear` (`self.HumanPaperToSpawn`)))

(fn `DestroyPaperPackage`
  (bind _tabofpaperpackage (`self.TabOfPaperPackage`))
  (for _array_element _tabofpaperpackage
    (`self.K2_DestroyActor` _array_element))
  (`KismetArrayLibrary.Array_Clear` _tabofpaperpackage)
  (`KismetArrayLibrary.Array_Clear` (`self.PackagePaperToSpawn`)))

(fn `DoesSaveGameExist?`
  (returns (ReturnValue :type Boolean))
  (bind _returnvalue (`GameplayStatics.DoesSaveGameExist` (`self.SlotName`)))
  (return _returnvalue))

(fn `HandleDifficulty`
  (switch `/Game/Essential/Difficulty_Enum` (`self.DifficultyMode`)
    (:`NewEnumerator0`
      (`TimelineComponent.SetPlayRate` (`self.DicreaseJaugePackage`) 0.0)
      (`TimelineComponent.SetPlayRate` (`self.DicreaseJaugeHuman`) 0.0)
      (set `self.FactorForBarPlus` 10.0)
      (set `self.FactorForBarMinus` 5.0))
    (:`NewEnumerator1`
      (`TimelineComponent.SetPlayRate` (`self.DicreaseJaugePackage`) 1.0)
      (`TimelineComponent.SetPlayRate` (`self.DicreaseJaugeHuman`) 1.0)
      (set `self.FactorForBarPlus` 10.0)
      (set `self.FactorForBarMinus` 5.0))
    (:`NewEnumerator2`
      (`TimelineComponent.SetPlayRate` (`self.DicreaseJaugePackage`) 2.0)
      (`TimelineComponent.SetPlayRate` (`self.DicreaseJaugeHuman`) 2.0)
      (set `self.FactorForBarPlus` 10.0)
      (set `self.FactorForBarMinus` 10.0))
    (:`NewEnumerator3`
      (`TimelineComponent.SetPlayRate` (`self.DicreaseJaugePackage`) 3.0)
      (`TimelineComponent.SetPlayRate` (`self.DicreaseJaugeHuman`) 3.0)
      (set `self.FactorForBarPlus` 5.0)
      (set `self.FactorForBarMinus` 10.0))))

(fn `HandleLoad`
  (bind _returnvalue (`GameplayStatics.LoadGameFromSlot` (`self.SlotName`)))
  (bind _asmy_save (cast `/Game/Essential/MySave` _returnvalue)
    (:`then`
      (set `self.CurrentDay` (`/Game/Essential/MySave.Day` _asmy_save))
      (set `self.HaveAlreadyFailed` (`/Game/Essential/MySave.AlreadyFail` _asmy_save))
      (set `self.DifficultyMode` (`/Game/Essential/MySave.DifficultyMode` _asmy_save)))
    (:`CastFailed`
      _))
  (return))

(fn `L'heureDeLaNews!`
  (bind _currentday (`self.CurrentDay`))
  (`GameplayStatics.SetGamePaused` true)
  (`|ExecutionSequence`
    (:`then_0`
      (bind _outrownames (`DataTableFunctionLibrary.GetDataTableRowNames` "/Game/Blueprints/Databases/Humans/BD_HumanEvents.BD_HumanEvents"))
      (for (_array_element _array_index) _outrownames
        (if (== (+ _array_index 1) _currentday)
          (bind _returnvalue (`|GetDataTableRow` "/Game/Blueprints/Databases/Humans/BD_HumanEvents.BD_HumanEvents" _array_element)
            (:`then`
              (set `self.EventHuman` (`KismetTextLibrary.Conv_StringToText` (`.Directive_6_12A0158A49A262A6CEA1A1969927B5AC` (break `/Game/Blueprints/Databases/Humans/STDT_HumanEvents` _returnvalue))))
              (`/Game/Essential/MyHUD.SetNews` (`self.HUDReference`) :!label _label))))))
    (:`then_1`
      (bind _outrownames_2 (`DataTableFunctionLibrary.GetDataTableRowNames` "/Game/Blueprints/Databases/Packages/BD_PackageEvents.BD_PackageEvents"))
      (for (_array_element_2 _array_index_2) _outrownames_2
        (if (== (+ _array_index_2 1) _currentday)
          (bind _returnvalue_2 (`|GetDataTableRow` "/Game/Blueprints/Databases/Packages/BD_PackageEvents.BD_PackageEvents" _array_element_2)
            (:`then`
              (set `self.EventPackage` (`KismetTextLibrary.Conv_StringToText` (`.Directive_6_12A0158A49A262A6CEA1A1969927B5AC` (break `/Game/Blueprints/Databases/Packages/STDT_PackageEvents` _returnvalue_2))))
              (goto _label))))))))

(fn `SaveMyGame`
  (bind _returnvalue (`GameplayStatics.CreateSaveGameObject` "/Game/Essential/MySave.MySave_C"))
  (bind _output_get (set `self.SaveRef` _returnvalue))
  (set `/Game/Essential/MySave.Day` (`self.CurrentDay`) _output_get)
  (set `/Game/Essential/MySave.AlreadyFail` (`self.HaveAlreadyFailed`) _output_get)
  (set `/Game/Essential/MySave.DifficultyMode` (`self.DifficultyMode`) _output_get)
  (`GameplayStatics.SaveGameToSlot` _output_get (`self.SlotName`)))

(fn `SpawnPaperHuman`
  (params (TheHuman :type "/Game/Blueprints/AI/Humans/HumanParent_BP Object Reference"))
  (bind (_haveid _havepp _havecs _havevisaw _havevisas _havevisat _haveaptitude _havepermis _haveassurance _havepermistravail _havediplome) (`/Game/Blueprints/AI/Humans/HumanParent_BP.GiveHumanParams` TheHuman))
  (bind _humanpapertospawn (`self.HumanPaperToSpawn`))
  (bind (_returnvalue_roll _returnvalue_pitch) (`KismetMathLibrary.BreakRotator` (`SceneComponent.K2_GetComponentRotation` (`self.Camera`))))
  (if _haveid
    (`KismetArrayLibrary.Array_AddUnique` _humanpapertospawn "/Game/Blueprints/AI/Papers/CarteDIdentite_BP.CarteDIdentite_BP_C"))
  (if _havepp
    (`KismetArrayLibrary.Array_AddUnique` _humanpapertospawn "/Game/Blueprints/AI/Papers/PassePort_BP.PassePort_BP_C"))
  (if _havecs
    (`KismetArrayLibrary.Array_AddUnique` _humanpapertospawn "/Game/Blueprints/AI/Papers/PapierCitoyennete_BP.PapierCitoyennete_BP_C"))
  (if _havevisaw
    (`KismetArrayLibrary.Array_AddUnique` _humanpapertospawn "/Game/Blueprints/AI/Papers/VisaTravail_BP.VisaTravail_BP_C"))
  (if _havevisas
    (`KismetArrayLibrary.Array_AddUnique` _humanpapertospawn "/Game/Blueprints/AI/Papers/VisaEtude_BP.VisaEtude_BP_C"))
  (if _havevisat
    (`KismetArrayLibrary.Array_AddUnique` _humanpapertospawn "/Game/Blueprints/AI/Papers/VisaVoyage_BP.VisaVoyage_BP_C"))
  (if _haveaptitude
    (`KismetArrayLibrary.Array_AddUnique` _humanpapertospawn "/Game/Blueprints/AI/Papers/CertificatDAptitude_BP.CertificatDAptitude_BP_C"))
  (if _havepermis
    (`KismetArrayLibrary.Array_AddUnique` _humanpapertospawn "/Game/Blueprints/AI/Papers/PermisDeSejour_BP.PermisDeSejour_BP_C"))
  (if _haveassurance
    (`KismetArrayLibrary.Array_AddUnique` _humanpapertospawn "/Game/Blueprints/AI/Papers/AttestationDAssurance_BP.AttestationDAssurance_BP_C"))
  (if _havepermistravail
    (`KismetArrayLibrary.Array_AddUnique` _humanpapertospawn "/Game/Blueprints/AI/Papers/PermisDeTravail_BP.PermisDeTravail_BP_C"))
  (if _havediplome
    (`KismetArrayLibrary.Array_AddUnique` _humanpapertospawn "/Game/Blueprints/AI/Papers/DiplomeDAptitude_BP.DiplomeDAptitude_BP_C"))
  (for (_array_element _array_index) (`self.HumanPaperToSpawn`)
    (bind (_returnvalue_x _returnvalue_y _returnvalue_z) (`KismetMathLibrary.BreakVector` (`SceneComponent.K2_GetComponentLocation` (select `bool` (>= _array_index 3) :`false` (`self.PlaceToSpawnHumanPapersTop`) :`true` (`self.PlaceToSpawnHumanPapersDown`)))))
    (bind _returnvalue (`|SpawnActorFromClass` _array_element (`KismetMathLibrary.MakeTransform` (`KismetMathLibrary.MakeVector` (+ (* (mod (`KismetMathLibrary.Conv_IntToDouble` _array_index) 3.0) 10.0) _returnvalue_x) _returnvalue_y _returnvalue_z) (`KismetMathLibrary.MakeRotator` _returnvalue_pitch (`KismetMathLibrary.RandomFloatInRange` -5.0 5.0)) (0.9 1.0 0.8)) "Undefined" "OverrideRootScale" self null))
    (`KismetArrayLibrary.Array_AddUnique` (`self.TabOfPaperHuman`) _returnvalue)))

(fn `SpawnPaperPackage`
  (params (TheBox :type "/Game/Blueprints/ConvoyerBelt/Boxes/BoxParent Object Reference"))
  (bind (_haveattestationacquittement _haveeori _havepasseportanimal _havedae _havespecialautorisation _haveeurmed _havevaccination _havecertifmedical _havesps) (`/Game/Blueprints/ConvoyerBelt/Boxes/BoxParent.GetPapers` TheBox))
  (bind _packagepapertospawn (`self.PackagePaperToSpawn`))
  (bind (_returnvalue_roll _returnvalue_pitch) (`KismetMathLibrary.BreakRotator` (`SceneComponent.K2_GetComponentRotation` (`self.Camera`))))
  (if _haveattestationacquittement
    (`KismetArrayLibrary.Array_AddUnique` _packagepapertospawn "/Game/Blueprints/ConvoyerBelt/Boxes/Papers/AttestationDAcquittement_BP.AttestationDAcquittement_BP_C"))
  (if _haveeori
    (`KismetArrayLibrary.Array_AddUnique` _packagepapertospawn "/Game/Blueprints/ConvoyerBelt/Boxes/Papers/NuméroEORI_BP.NuméroEORI_BP_C"))
  (if _havepasseportanimal
    (`KismetArrayLibrary.Array_AddUnique` _packagepapertospawn "/Game/Blueprints/ConvoyerBelt/Boxes/Papers/PassePortAnimal_BP.PassePortAnimal_BP_C"))
  (if _havedae
    (`KismetArrayLibrary.Array_AddUnique` _packagepapertospawn "/Game/Blueprints/ConvoyerBelt/Boxes/Papers/DocumentDAccompegnementElectronique_BP.DocumentDAccompegnementElectronique_BP_C"))
  (if _havespecialautorisation
    (`KismetArrayLibrary.Array_AddUnique` _packagepapertospawn "/Game/Blueprints/ConvoyerBelt/Boxes/Papers/AutorisationSpeciale_BP.AutorisationSpeciale_BP_C"))
  (if _haveeurmed
    (`KismetArrayLibrary.Array_AddUnique` _packagepapertospawn "/Game/Blueprints/ConvoyerBelt/Boxes/Papers/CertificatEURMED_BP.CertificatEURMED_BP_C"))
  (if _havevaccination
    (`KismetArrayLibrary.Array_AddUnique` _packagepapertospawn "/Game/Blueprints/ConvoyerBelt/Boxes/Papers/CertificatVaccination_BP.CertificatVaccination_BP_C"))
  (if _havecertifmedical
    (`KismetArrayLibrary.Array_AddUnique` _packagepapertospawn "/Game/Blueprints/ConvoyerBelt/Boxes/Papers/CertificatMedical_BP.CertificatMedical_BP_C"))
  (if _havesps
    (`KismetArrayLibrary.Array_AddUnique` _packagepapertospawn "/Game/Blueprints/ConvoyerBelt/Boxes/Papers/SPS_BP.SPS_BP_C"))
  (for (_array_element _array_index) (`self.PackagePaperToSpawn`)
    (bind (_returnvalue_x _returnvalue_y _returnvalue_z) (`KismetMathLibrary.BreakVector` (`SceneComponent.K2_GetComponentLocation` (select `bool` (>= _array_index 3) :`false` (`self.PlaceToSpawnPackagesPapersTop`) :`true` (`self.PlaceToSpawnPackagesPapersDown`)))))
    (bind _returnvalue (`|SpawnActorFromClass` _array_element (`KismetMathLibrary.MakeTransform` (`KismetMathLibrary.MakeVector` (+ (* (mod (`KismetMathLibrary.Conv_IntToDouble` _array_index) 3.0) 10.0) _returnvalue_x) _returnvalue_y _returnvalue_z) (`KismetMathLibrary.MakeRotator` _returnvalue_pitch (`KismetMathLibrary.RandomFloatInRange` -5.0 5.0)) (0.9 1.0 0.8)) "Undefined" "OverrideRootScale" self null))
    (`KismetArrayLibrary.Array_AddUnique` (`self.TabOfPaperPackage`) _returnvalue)))

(fn `UserConstructionScript`)