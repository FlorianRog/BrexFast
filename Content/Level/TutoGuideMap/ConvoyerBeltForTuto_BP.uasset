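; Tutorial conveyor belt that carries spawned packages to an inspection zone for the player to accept or reject.
; Tick moves overlapping boxes along the belt until one enters InTraitment, which pauses the belt, centers the box and shows its paperwork through the player pawn.
; Yes pushes the box sideways and No springs it upward; both clear the paperwork, update the package gauge based on IsAGoodBox and restart the belt.
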(event `self.ReceiveBeginPlay`
  ;[1 1 1] Set a few variables
  (bind _asthe_player_camera_for_tuto_bp (cast `/Game/Level/TutoGuideMap/ThePlayerCameraForTuto_BP` (`GameplayStatics.GetPlayerPawn` 0)))
  (bind _output_get (set `self.ThePlayer` _asthe_player_camera_for_tuto_bp))
  (set `/Game/Level/TutoGuideMap/ThePlayerCameraForTuto_BP.TheCarpet` self _output_get)
  (set `self.TheDirection` (`self.NormalDirection`))
  (set `self.BoxForMovements` (`self.NormalMovementBox`))
  (bind _asspring_bp (cast `/Game/Blueprints/Spring/Spring_Bp` (`ChildActorComponent.ChildActor` (`self.Spring`))))
  (set `self.MySpring` _asspring_bp))

(event `SpawnBoxes`
  (params (GoodBox :type Boolean))
  ;[1 1 1] Set timer for spawing boxes
  (bind _returnvalue (`|SpawnActorFromClass` "/Game/Level/TutoGuideMap/BoxParentForTuto.BoxParentForTuto_C" (`SceneComponent.K2_GetComponentToWorld` (`self.PlaceToSpawn`)) "Undefined" "OverrideRootScale" null GoodBox null))
  (set `self.SpawnedBox` _returnvalue))

(event `self.ReceiveTick`
  (params (DeltaSeconds :type "Float (single-precision)"))
  ;[1 1 1] Adding movement to the convoyer belt
  (for _array_element (`PrimitiveComponent.GetOverlappingActors` (`self.BoxForMovements`) "/Game/Blueprints/ConvoyerBelt/Boxes/BoxParent.BoxParent_C")
    (if (!= _array_element self)
      (`self.K2_AddActorWorldOffset` _array_element (* (`SceneComponent.GetForwardVector` (`self.TheDirection`)) (* DeltaSeconds (`self.Speed`))) false false))))

(event `self.InTraitment.OnComponentBeginOverlap`
  (params (OverlappedComponent :type "PrimitiveComponent Object Reference") (OtherActor :type "Actor Object Reference") (OtherComp :type "PrimitiveComponent Object Reference") (OtherBodyIndex :type Integer) (bFromSweep :type Boolean) (SweepResult :type "HitResult Structure (by ref)"))
  (bind _theplayer (`self.ThePlayer`))
  ;[1 1 1] On traitement box overlap, move the box to the center and disable the convoyer belt movement
  (if (!= OtherActor (`self.TheBox`))
    (bind _asbox_parent (cast `/Game/Blueprints/ConvoyerBelt/Boxes/BoxParent` OtherActor))
    (set `self.CanSpawn` false)
    (bind _output_get (set `self.TheBox` _asbox_parent))
    (`self.SetActorTickEnabled` false)
    (`/Game/Level/TutoGuideMap/ThePlayerCameraForTuto_BP.SpawnPaperPackage` _theplayer _output_get)
    (`/Game/Level/TutoGuideMap/ThePlayerCameraForTuto_BP.SpawnPackageInfos` _theplayer (`/Game/Blueprints/ConvoyerBelt/Boxes/BoxParent.PackageType` _output_get) (`/Game/Blueprints/ConvoyerBelt/Boxes/BoxParent.From` _output_get))
    (`KismetSystemLibrary.MoveComponentTo` (`/Game/Blueprints/ConvoyerBelt/Boxes/BoxParent.TheBox` _output_get) (`SceneComponent.K2_GetComponentLocation` (`self.InTraitment`)))
    (`/Engine/EditorBlueprintResources/StandardMacros.DoOnce` false
      (:`Completed`
        (`/Game/Level/TutoGuideMap/ThePlayerCameraForTuto_BP.BaisseJaugePackage` (`self.ThePlayer`))))))

(fn `No`
  (bind _thebox (`self.TheBox`))
  (bind _theplayer (`self.ThePlayer`))
  (`/Game/Level/TutoGuideMap/ThePlayerCameraForTuto_BP.DestroyPaperPackage` _theplayer)
  (`/Game/Level/TutoGuideMap/ThePlayerCameraForTuto_BP.DestroyPackageDescription` _theplayer)
  (`/Engine/EditorBlueprintResources/StandardMacros.IsValid` _thebox
    (:`Is Valid`
      (`/Game/Level/TutoGuideMap/ThePlayerCameraForTuto_BP.ChangeJaugePackage` (`self.ThePlayer`) (`/Game/Blueprints/ConvoyerBelt/Boxes/BoxParent.IsAGoodBox` _thebox))
      (`/Game/Blueprints/Spring/Spring_Bp.Boing` (`self.MySpring`))
      (`PrimitiveComponent.AddImpulse` (`/Game/Blueprints/ConvoyerBelt/Boxes/BoxParent.TheBox` (`self.TheBox`)) (0.0 0.0 5000000.0) "None" false)
      (`self.SetActorTickEnabled` true)
      (set `self.CanSpawn` true))))

(fn `UserConstructionScript`)

(fn `Yes`
  (bind _thebox (`self.TheBox`))
  (bind _theplayer (`self.ThePlayer`))
  (`/Game/Level/TutoGuideMap/ThePlayerCameraForTuto_BP.DestroyPaperPackage` _theplayer)
  (`/Game/Level/TutoGuideMap/ThePlayerCameraForTuto_BP.DestroyPackageDescription` _theplayer)
  (`/Engine/EditorBlueprintResources/StandardMacros.IsValid` _thebox
    (:`Is Valid`
      (`/Game/Level/TutoGuideMap/ThePlayerCameraForTuto_BP.ChangeJaugePackage` (`self.ThePlayer`) (not (`/Game/Blueprints/ConvoyerBelt/Boxes/BoxParent.IsAGoodBox` _thebox)))
      (`PrimitiveComponent.AddImpulse` (`/Game/Blueprints/ConvoyerBelt/Boxes/BoxParent.TheBox` (`self.TheBox`)) (-2500000.0 0.0 0.0) "None" false)
      (`self.SetActorTickEnabled` true)
      (set `self.CanSpawn` true))))