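; Tutorial-map human parent: a randomized traveler who waits in the spawner's line of target points and carries an identity profile.
; Construction script randomizes sex, mesh, skin, clothing and hair materials.
; BeginPlay rolls travel type, duration and first name from data tables, then sets ID or passport flags and good-human status from ShouldSpawnGoodHuman.
; Move advances it to an unblocked free slot or to the destroy box, and clicks notify the anim instance of head hits.
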(event `SetIsGiving`
  (message `/Game/Assets/Humans/Animations/Anim_I.IsGiving` (`SkeletalMeshComponent.GetAnimInstance` (`self.Mesh`))))

(event `/Game/Blueprints/ClickedEvent.Clicked`
  (params (Component :type "ActorComponent Object Reference"))
  (message `/Game/Assets/Humans/Animations/Anim_I.IsHit` (`SkeletalMeshComponent.GetAnimInstance` (`self.Mesh`)) (== Component (`self.headSphere`))))

(event `self.ReceiveBeginPlay`
  (bind _asplayer_controller (cast `/Game/Essential/PlayerController` (`GameplayStatics.GetPlayerController` 0)))
  (bind _output_get (set `self.ThePlayerInformation` _asplayer_controller))
  (bind _output_get_2 (set `self.MyHumanSpawner` (`/Game/Essential/PlayerController.TheHuman` _output_get)))
  (set `self.CurrentTargetPointIndex` (`KismetArrayLibrary.Array_LastIndex` (`/Game/Blueprints/AI/HumanSpawner_BP.TargetPoints` _output_get_2)))
  ;[1 1 1] Set the travel type
  (bind _outrownames (`DataTableFunctionLibrary.GetDataTableRowNames` "/Game/Blueprints/Databases/Humans/DB_TravelType.DB_TravelType"))
  (set `self.RandomTravelTypeID` (`KismetMathLibrary.RandomIntegerInRange` 0 (- (`KismetArrayLibrary.Array_Length` _outrownames) 1)))
  (for (_array_element _array_index) _outrownames
    (if (== _array_index (`self.RandomTravelTypeID`))
      (bind _returnvalue (`|GetDataTableRow` "/Game/Blueprints/Databases/Humans/DB_TravelType.DB_TravelType" _array_element)
        (:`then`
          (bind (_traveltype _isaworker _isastudent _isatraveler _isamigrant) (break `/Game/Blueprints/Databases/Humans/STDT_TravelType` _returnvalue))
          (set `self.TravelType` _traveltype)
          (set `self.IsAWorker` _isaworker)
          (set `self.IsAStudent` _isastudent)
          (set `self.IsATraveler` _isatraveler)
          (set `self.IsAMigrant` _isamigrant)))))
  (if (`self.IsAMigrant`)
    (set `self.Duration` "Toujours")
    (set `self.IsALongJourney` true)
    (else
      ;[1 1 1] Get a duration
      (bind _outrownames_2 (`DataTableFunctionLibrary.GetDataTableRowNames` "/Game/Blueprints/Databases/Humans/BD_Duration.BD_Duration"))
      (set `self.RandomDurationID` (`KismetMathLibrary.RandomIntegerInRange` 0 (- (`KismetArrayLibrary.Array_Length` _outrownames_2) 1)))
      (for (_array_element_2 _array_index_2) _outrownames_2
        (if (== _array_index_2 (`self.RandomDurationID`))
          (bind _returnvalue_2 (`|GetDataTableRow` "/Game/Blueprints/Databases/Humans/BD_Duration.BD_Duration" _array_element_2)
            (:`then`
              (bind (_duration _islong) (break `/Game/Blueprints/Databases/Humans/STDT_Duration` _returnvalue_2))
              (set `self.Duration` _duration)
              (set `self.IsALongJourney` _islong)))))))
  ;[1 1 1] Pick a random name
  (if (`self.IsMale`)
    (bind _outrownames_3 (`DataTableFunctionLibrary.GetDataTableRowNames` "/Game/Blueprints/Databases/Humans/BD_PrenomMale.BD_PrenomMale"))
    (set `self.RandomNameID` (- (`KismetMathLibrary.RandomIntegerInRange` 0 (`KismetArrayLibrary.Array_Length` _outrownames_3)) 1))
    (for (_array_element_3 _array_index_3) _outrownames_3
      (if (== _array_index_3 (`self.RandomNameID`))
        (bind _returnvalue_3 (`|GetDataTableRow` "/Game/Blueprints/Databases/Humans/BD_PrenomMale.BD_PrenomMale" _array_element_3)
          (:`then`
            (set `self.Prenom` (`.Prenom_5_923AD7C849F9D4EE403BC28E32FA6A51` (break `/Game/Blueprints/Databases/Humans/STDT_PrenomMale` _returnvalue_3)))))))
    (else
      (bind _outrownames_4 (`DataTableFunctionLibrary.GetDataTableRowNames` "/Game/Blueprints/Databases/Humans/BD_PrenomFemale.BD_PrenomFemale"))
      (set `self.RandomNameID` (- (`KismetMathLibrary.RandomIntegerInRange` 0 (`KismetArrayLibrary.Array_Length` _outrownames_4)) 1))
      (for (_array_element_4 _array_index_4) _outrownames_4
        (if (== _array_index_4 (`self.RandomNameID`))
          (bind _returnvalue_4 (`|GetDataTableRow` "/Game/Blueprints/Databases/Humans/BD_PrenomFemale.BD_PrenomFemale" _array_element_4)
            (:`then`
              (set `self.Prenom` (`.Prenom_5_923AD7C849F9D4EE403BC28E32FA6A51` (break `/Game/Blueprints/Databases/Humans/STDT_PrenomFemale` _returnvalue_4)))))))))
  (`self.CheckIDPapers`))

(event `SetGoodHuman`
  ;[1 1 1] Directive change stat
  ;;[1 1 1] Set is a good human
  (for _array_element (`self.IsInGoodWay`)
    (set `self.IsAGoodHuman` (and _array_element (`self.IsAGoodHuman`)))))

(event `CheckIDPapers`
  (bind _isingoodway (`self.IsInGoodWay`))
  ;[1 1 1] Directive change stat
  ;;[1 1 1] CheckIDPapers
  (if (`self.ShouldSpawnGoodHuman`)
    (bind _output_get (set `self.HaveID` (`KismetMathLibrary.RandomBool`)))
    (set `self.HavePP` (not _output_get))
    (`KismetArrayLibrary.Array_Add` _isingoodway true)
    (else
      (set `self.HaveID` false)
      (set `self.HavePP` false)
      (`KismetArrayLibrary.Array_Add` _isingoodway)))
  (`self.SetGoodHuman`))

(event `Move`
  (params (ToDeath :type Boolean))
  (bind _myhumanspawner (`self.MyHumanSpawner`))
  (if ToDeath
    (`KismetSystemLibrary.MoveComponentTo` (`self.RootComponent`) (`SceneComponent.K2_GetComponentLocation` (`/Game/Blueprints/AI/HumanSpawner_BP.BoxForDestroy` (`self.MyHumanSpawner`))))
    (else
      ;[1 1 1] Explore the tab of target points occuped and check that the index is smaller than its own but also that the place is not already taken
      (for _index (range (`self.CurrentTargetPointIndex`))
        (set `self.NewIndex` _index)
        (if (not (`|GetArrayItem` (`/Game/Blueprints/AI/HumanSpawner_BP.TargetPointsOccuped` (`self.MyHumanSpawner`)) (`self.NewIndex`)))
          ;[1 1 1] Check if there is an already taken place between the human current's place and its target
          (for _index_2 (range (`self.NewIndex`) (`self.CurrentTargetPointIndex`))
            (set `self.SomethingBetweenIndexes` (or (`self.SomethingBetweenIndexes`) (`|GetArrayItem` (`/Game/Blueprints/AI/HumanSpawner_BP.TargetPointsOccuped` (`self.MyHumanSpawner`)) _index_2))))
          (if (not (`self.SomethingBetweenIndexes`))
            (set `self.PlaceFound` true)
            (break))))
      ;[1 1 1] Check if a place was found
      (if (`self.PlaceFound`)
        ;[1 1 1] Change the availability of the places
        (`KismetArrayLibrary.Array_Set` (`/Game/Blueprints/AI/HumanSpawner_BP.TargetPointsOccuped` (`self.MyHumanSpawner`)) (`self.CurrentTargetPointIndex`))
        (set `self.CurrentTargetPointIndex` (`self.NewIndex`))
        (`KismetArrayLibrary.Array_Set` (`/Game/Blueprints/AI/HumanSpawner_BP.TargetPointsOccuped` (`self.MyHumanSpawner`)) (`self.CurrentTargetPointIndex`) true)
        ;[1 1 1] Set the location to go
        (`|AIMoveTo` self (`KismetMathLibrary.TransformLocation` (`self.GetTransform` _myhumanspawner) (`|GetArrayItem` (`/Game/Blueprints/AI/HumanSpawner_BP.TargetPoints` _myhumanspawner) (`self.CurrentTargetPointIndex`))) null)))))

(fn `GiveHumanParams`
  (returns (HaveID :type Boolean) (HavePP :type Boolean))
  (return (`self.HaveID`) (`self.HavePP`)))

(fn `IsNextTargetPointFree`
  (returns (NewParam :type Boolean))
  (return false))

(fn `UserConstructionScript`
  (bind _mesh (`self.Mesh`))
  (bind _mesh_2 (`self.Mesh`))
  (bind _mesh_3 (`self.Mesh`))
  (bind _mesh_4 (`self.Mesh`))
  (bind _mesh_5 (`self.Mesh`))
  (bind _mesh_6 (`self.Mesh`))
  (bind _mesh_7 (`self.Mesh`))
  (if (`KismetMathLibrary.RandomBool`)
    (`SkinnedMeshComponent.SetSkinnedAssetAndUpdate` _mesh_4 "/Game/Assets/Humans/Male/Male.Male" true)
    (set `self.IsMale` true)
    ;[1 1 1] Change la couleur de la peau
    (`PrimitiveComponent.SetMaterial` (`self.Mesh`) 0 "/Game/Assets/MaterialAndTextures/Materiaux/BaseTexture/BT_Parent.BT_Parent")
    ;[1 1 1] Change la couleur du tshirt
    (switch `int` (`KismetMathLibrary.RandomIntegerInRange` 0 4)
      (:`Default`
        (`PrimitiveComponent.SetMaterial` _mesh_3 1 "/Game/Assets/MaterialAndTextures/Materiaux/BaseColor/Childs/inst_f7f1e3.inst_f7f1e3" :!label _label))
      (:`0`
        (`PrimitiveComponent.SetMaterial` _mesh_3 1 "/Game/Assets/MaterialAndTextures/Materiaux/BaseColor/Childs/inst_84817a.inst_84817a"))
      (:`1`
        (`PrimitiveComponent.SetMaterial` _mesh_3 1 "/Game/Assets/MaterialAndTextures/Materiaux/BaseColor/Childs/inst_34ace0.inst_34ace0"))
      (:`2`
        (`PrimitiveComponent.SetMaterial` _mesh_3 1 "/Game/Assets/MaterialAndTextures/Materiaux/BaseColor/Childs/inst_ccae62.inst_ccae62"))
      (:`3`
        (`PrimitiveComponent.SetMaterial` _mesh_3 1 "/Game/Assets/MaterialAndTextures/Materiaux/BaseColor/Childs/inst_ff5252.inst_ff5252"))
      (:`4`
        (goto _label)))
    ;[1 1 1] Change la couleur du pantalon
    (switch `int` (`KismetMathLibrary.RandomIntegerInRange` 0 3)
      (:`Default`
        (`PrimitiveComponent.SetMaterial` _mesh 2 "/Game/Assets/MaterialAndTextures/Materiaux/BaseColor/Childs/inst_d1ccc0.inst_d1ccc0" :!label _label_2))
      (:`0`
        (`PrimitiveComponent.SetMaterial` _mesh 2 "/Game/Assets/MaterialAndTextures/Materiaux/BaseColor/Childs/inst_84817a.inst_84817a"))
      (:`1`
        (`PrimitiveComponent.SetMaterial` _mesh 2 "/Game/Assets/MaterialAndTextures/Materiaux/BaseColor/Childs/inst_34ace0.inst_34ace0"))
      (:`2`
        (`PrimitiveComponent.SetMaterial` _mesh 2 "/Game/Assets/MaterialAndTextures/Materiaux/BaseColor/Childs/inst_f7f1e3.inst_f7f1e3"))
      (:`3`
        (goto _label_2)))
    (else
      (`SkinnedMeshComponent.SetSkinnedAssetAndUpdate` _mesh_4 "/Game/Assets/Humans/Female/Female.Female" true)
      (set `self.IsMale` false)
      ;[1 1 1] Change la couleur de la peau
      (`PrimitiveComponent.SetMaterial` (`self.Mesh`) 0 "/Game/Assets/MaterialAndTextures/Materiaux/BaseTexture/BT_Parent.BT_Parent")
      ;[1 1 1] Change la couleur du tshirt
      (switch `int` (`KismetMathLibrary.RandomIntegerInRange` 0 9)
        (:`Default`
          (`PrimitiveComponent.SetMaterial` _mesh_5 1 "/Game/Assets/MaterialAndTextures/Materiaux/BaseColor/Childs/inst_ffb142.inst_ffb142" :!label _label_3))
        (:`0`
          (`PrimitiveComponent.SetMaterial` _mesh_5 1 "/Game/Assets/MaterialAndTextures/Materiaux/BaseColor/Childs/inst_84817a.inst_84817a"))
        (:`1`
          (`PrimitiveComponent.SetMaterial` _mesh_5 1 "/Game/Assets/MaterialAndTextures/Materiaux/BaseColor/Childs/inst_34ace0.inst_34ace0"))
        (:`2`
          (`PrimitiveComponent.SetMaterial` _mesh_5 1 "/Game/Assets/MaterialAndTextures/Materiaux/BaseColor/Childs/inst_ccae62.inst_ccae62"))
        (:`3`
          (`PrimitiveComponent.SetMaterial` _mesh_5 1 "/Game/Assets/MaterialAndTextures/Materiaux/BaseColor/Childs/inst_218c74.inst_218c74"))
        (:`4`
          (`PrimitiveComponent.SetMaterial` _mesh_5 1 "/Game/Assets/MaterialAndTextures/Materiaux/BaseColor/Childs/inst_ff793f.inst_ff793f"))
        (:`5`
          (`PrimitiveComponent.SetMaterial` _mesh_5 1 "/Game/Assets/MaterialAndTextures/Materiaux/BaseColor/Childs/inst_706fd3.inst_706fd3"))
        (:`6`
          (`PrimitiveComponent.SetMaterial` _mesh_5 1 "/Game/Assets/MaterialAndTextures/Materiaux/BaseColor/Childs/inst_474787.inst_474787"))
        (:`7`
          (`PrimitiveComponent.SetMaterial` _mesh_5 1 "/Game/Assets/MaterialAndTextures/Materiaux/BaseColor/Childs/inst_b33939.inst_b33939"))
        (:`8`
          (`PrimitiveComponent.SetMaterial` _mesh_5 1 "/Game/Assets/MaterialAndTextures/Materiaux/BaseColor/Childs/inst_f7f1e3.inst_f7f1e3"))
        (:`9`
          (goto _label_3)))
      ;[1 1 1] Change la couleur du pantalon
      (switch `int` (`KismetMathLibrary.RandomIntegerInRange` 0 3)
        (:`Default`
          (`PrimitiveComponent.SetMaterial` _mesh_6 2 "/Game/Assets/MaterialAndTextures/Materiaux/BaseColor/Childs/inst_ffb142.inst_ffb142" :!label _label_4))
        (:`0`
          (`PrimitiveComponent.SetMaterial` _mesh_6 2 "/Game/Assets/MaterialAndTextures/Materiaux/BaseColor/Childs/inst_34ace0.inst_34ace0"))
        (:`1`
          (`PrimitiveComponent.SetMaterial` _mesh_6 2 "/Game/Assets/MaterialAndTextures/Materiaux/BaseColor/Childs/inst_b33939.inst_b33939"))
        (:`2`
          (`PrimitiveComponent.SetMaterial` _mesh_6 2 "/Game/Assets/MaterialAndTextures/Materiaux/BaseColor/Childs/inst_f7f1e3.inst_f7f1e3"))
        (:`3`
          (goto _label_4)))))
  ;[1 1 1] Change la couleur des chaussures
  (switch `int` (`KismetMathLibrary.RandomIntegerInRange` 0 2)
    (:`Default`
      (`PrimitiveComponent.SetMaterial` _mesh_7 3 "/Game/Assets/MaterialAndTextures/Materiaux/BaseColor/Childs/inst_f7f1e3.inst_f7f1e3" :!label _label_5))
    (:`0`
      (`PrimitiveComponent.SetMaterial` _mesh_7 3 "/Game/Assets/MaterialAndTextures/Materiaux/BaseColor/Childs/inst_84817a.inst_84817a"))
    (:`1`
      (`PrimitiveComponent.SetMaterial` _mesh_7 3 "/Game/Assets/MaterialAndTextures/Materiaux/BaseColor/Childs/inst_ccae62.inst_ccae62"))
    (:`2`
      (goto _label_5)))
  ;[1 1 1] Change la couleur des cheveux
  (switch `int` (`KismetMathLibrary.RandomIntegerInRange` 0 5)
    (:`Default`
      (`PrimitiveComponent.SetMaterial` _mesh_2 4 "/Game/Assets/MaterialAndTextures/Materiaux/BaseColor/Childs/inst_ff793f.inst_ff793f" :!label _label_6))
    (:`0`
      (`PrimitiveComponent.SetMaterial` _mesh_2 4 "/Game/Assets/MaterialAndTextures/Materiaux/BaseColor/Childs/inst_2c2c54.inst_2c2c54"))
    (:`1`
      (`PrimitiveComponent.SetMaterial` _mesh_2 4 "/Game/Assets/MaterialAndTextures/Materiaux/BaseColor/Childs/inst_ffb142.inst_ffb142"))
    (:`2`
      (`PrimitiveComponent.SetMaterial` _mesh_2 4 "/Game/Assets/MaterialAndTextures/Materiaux/BaseColor/Childs/inst_227093.inst_227093"))
    (:`3`
      (`PrimitiveComponent.SetMaterial` _mesh_2 4 "/Game/Assets/MaterialAndTextures/Materiaux/BaseColor/Childs/inst_cd6133.inst_cd6133"))
    (:`4`
      (`PrimitiveComponent.SetMaterial` _mesh_2 4 "/Game/Assets/MaterialAndTextures/Materiaux/BaseColor/Childs/inst_b33939.inst_b33939"))
    (:`5`
      (goto _label_6)))
  (switch `int` (`KismetMathLibrary.RandomIntegerInRange` 0 16)
    (:`0`
      (set `self.MaterialForSkin` "/Game/Assets/MaterialAndTextures/Materiaux/BaseTexture/Childs/Skins/BT_Skin1.BT_Skin1"))
    (:`1`
      (set `self.MaterialForSkin` "/Game/Assets/MaterialAndTextures/Materiaux/BaseTexture/Childs/Skins/BT_Skin2.BT_Skin2"))
    (:`2`
      (set `self.MaterialForSkin` "/Game/Assets/MaterialAndTextures/Materiaux/BaseTexture/Childs/Skins/BT_Skin3.BT_Skin3"))
    (:`3`
      (set `self.MaterialForSkin` "/Game/Assets/MaterialAndTextures/Materiaux/BaseTexture/Childs/Skins/BT_Skin4.BT_Skin4"))
    (:`4`
      (set `self.MaterialForSkin` "/Game/Assets/MaterialAndTextures/Materiaux/BaseTexture/Childs/Skins/BT_Skin5.BT_Skin5"))
    (:`5`
      (set `self.MaterialForSkin` "/Game/Assets/MaterialAndTextures/Materiaux/BaseTexture/Childs/Skins/BT_Skin6.BT_Skin6"))
    (:`6`
      (set `self.MaterialForSkin` "/Game/Assets/MaterialAndTextures/Materiaux/BaseTexture/Childs/Skins/BT_Skin7.BT_Skin7"))
    (:`7`
      (set `self.MaterialForSkin` "/Game/Assets/MaterialAndTextures/Materiaux/BaseTexture/Childs/Skins/BT_Skin8.BT_Skin8"))
    (:`8`
      (set `self.MaterialForSkin` "/Game/Assets/MaterialAndTextures/Materiaux/BaseTexture/Childs/Skins/BT_Skin9.BT_Skin9"))
    (:`9`
      (set `self.MaterialForSkin` "/Game/Assets/MaterialAndTextures/Materiaux/BaseTexture/Childs/Skins/BT_Skin10.BT_Skin10"))
    (:`10`
      (set `self.MaterialForSkin` "/Game/Assets/MaterialAndTextures/Materiaux/BaseTexture/Childs/Skins/BT_Skin11.BT_Skin11"))
    (:`11`
      (set `self.MaterialForSkin` "/Game/Assets/MaterialAndTextures/Materiaux/BaseTexture/Childs/Skins/BT_Skin12.BT_Skin12"))
    (:`12`
      (set `self.MaterialForSkin` "/Game/Assets/MaterialAndTextures/Materiaux/BaseTexture/Childs/Skins/BT_Skin13.BT_Skin13"))
    (:`13`
      (set `self.MaterialForSkin` "/Game/Assets/MaterialAndTextures/Materiaux/BaseTexture/Childs/Skins/BT_Skin14.BT_Skin14"))
    (:`14`
      (set `self.MaterialForSkin` "/Game/Assets/MaterialAndTextures/Materiaux/BaseTexture/Childs/Skins/BT_Skin15.BT_Skin15"))
    (:`15`
      (set `self.MaterialForSkin` "/Game/Assets/MaterialAndTextures/Materiaux/BaseTexture/Childs/Skins/BT_Skin16.BT_Skin16"))
    (:`16`
      (set `self.MaterialForSkin` "/Game/Assets/MaterialAndTextures/Materiaux/BaseTexture/Childs/Skins/BT_Skin17.BT_Skin17")))
  (`PrimitiveComponent.SetMaterial` (`self.Mesh`) 0 (`self.MaterialForSkin`)))