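; Tutorial player camera for a document-checking game, presenting papers and descriptions of humans and packages.
; Interface events spawn and destroy paper actors from each subject's document flags, laid out in two camera-tilted rows.
; Timelines slide description cards in and out and run human and package gauges that end in game over.
; Right or wrong answers play a sound and shift the gauges, with drain rate and adjustments set by difficulty.
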(event `self.ReceiveBeginPlay`
  (bind _asmy_player_controller (cast `/Game/Essential/MyPlayerController` (`GameplayStatics.GetPlayerController` 0)))
  (set `self.MyPlayerController` _asmy_player_controller))

(event `PlayAnimationDescriptionHuman`
  (if (`self.HumanDescriptionHidden?`) :!label _label
    (set `self.HumanDescriptionHidden?` false)
    (bind (_direction _alpha) (`Timeline|SpawnHumanDescription` :!label _label_2)
      (:`Update`
        (`SceneComponent.K2_SetWorldLocation` (`/Game/Blueprints/UserInterface/HumanDescription_BP.Plane` (`self.TheHumanDescription`)) (`KismetMathLibrary.VLerp` (`SceneComponent.K2_GetComponentLocation` (`self.PlaceToSpawnHumanDescription`)) (`SceneComponent.K2_GetComponentLocation` (`self.PlaceWhereHumanDescriptionNeedToGo`)) _alpha) false false)))
    (else
      (set `self.HumanDescriptionHidden?` true)
      (goto _label_2 :!via `Reverse`))))

(event `PlayAnimationDescriptionPackage`
  (if (`self.PackageDescriptionHidden`) :!label _label_3
    (set `self.PackageDescriptionHidden` false)
    (bind (_direction _alpha) (`Timeline|SpawnPackageDescription` :!label _label_4)
      (:`Update`
        (`SceneComponent.K2_SetWorldLocation` (`/Game/Blueprints/UserInterface/PackageDescription_BP.Plane` (`self.ThePackageDescription`)) (`KismetMathLibrary.VLerp` (`SceneComponent.K2_GetComponentLocation` (`self.PlaceToSpawnPackageDescription`)) (`SceneComponent.K2_GetComponentLocation` (`self.PlaceWherePackageDescriptionNeedToGo`)) _alpha) false false)))
    (else
      (set `self.PackageDescriptionHidden` true)
      (goto _label_4 :!via `Reverse`))))

(event `/Game/Essential/PCToPawn_I.HandleDifficulty_I`
  (params (Difficulty :type "/Game/Essential/Difficulty_Enum Enum" :default "NewEnumerator0"))
  (`self.HandleDifficultyMode` Difficulty))

(event `/Game/Essential/PCToPawn_I.BaisseJaugePackage_I`
  (bind (_direction _alpha) (`Timeline|DicreaseJaugePackage` :`NewTime` (- 100.0 (stale `/Game/Essential/PCToPawn_I.ChangeJaugePackage_I` _output_get)) :!label _label_5)
    (:`Update`
      (set `self.TimePackage` _alpha))
    (:`Finished`
      (`/Game/Essential/MyPlayerController.EndGameGameOver` (`self.MyPlayerController`)))))

(event `/Game/Essential/PCToPawn_I.BaisseJaugeHuman_I`
  (bind (_direction _alpha) (`Timeline|DicreaseJaugeHuman` :`NewTime` (- 100.0 (stale `/Game/Essential/PCToPawn_I.ChangeJaugeHuman_I` _output_get)) :!label _label_6)
    (:`Update`
      (set `self.TimeHuman` _alpha))
    (:`Finished`
      (`/Game/Essential/MyPlayerController.EndGameGameOver` (`self.MyPlayerController`)))))

(event `/Game/Essential/PCToPawn_I.ChangeJaugePackage_I`
  (params (Error :type Boolean))
  (bind _timepackage (`self.TimePackage`))
  (if Error
    (`GameplayStatics.PlaySound2D` "/Game/Assets/Sounds/Faux.Faux" 1.0 1.0 0.0 null null)
    (else
      (`GameplayStatics.PlaySound2D` "/Game/Assets/Sounds/Correct_1.Correct_1" 1.0 1.0 0.0 null null)))
  (bind _output_get (set `self.TimePackage` (`KismetMathLibrary.FClamp` (select `bool` Error :`false` (+ _timepackage (`self.FactorForBarPlus`)) :`true` (- _timepackage (`self.FactorForBarMinus`))) 0.0 100.0)))
  (goto _label_5 :!via `SetNewTime`))

(event `/Game/Essential/PCToPawn_I.ChangeJaugeHuman_I`
  (params (Error :type Boolean))
  (bind _timehuman (`self.TimeHuman`))
  (if Error
    (`GameplayStatics.PlaySound2D` "/Game/Assets/Sounds/Faux.Faux" 1.0 1.0 0.0 null null)
    (else
      (`GameplayStatics.PlaySound2D` "/Game/Assets/Sounds/Correct_1.Correct_1" 1.0 1.0 0.0 null null)))
  (bind _output_get (set `self.TimeHuman` (`KismetMathLibrary.FClamp` (select `bool` Error :`false` (+ _timehuman (`self.FactorForBarPlus`)) :`true` (- _timehuman (`self.FactorForBarMinus`))) 0.0 100.0)))
  (goto _label_6 :!via `SetNewTime`))

(event `/Game/Essential/PCToPawn_I.SpawnHumanInfo_I`
  (params (Name :type String) (TravelType :type String) (JourneyDuration :type String))
  (bind _returnvalue (`|SpawnActorFromClass` "/Game/Blueprints/UserInterface/HumanDescription_BP.HumanDescription_BP_C" (`SceneComponent.K2_GetComponentToWorld` (`self.PlaceToSpawnHumanDescription`)) "Undefined" "OverrideRootScale" null Name TravelType JourneyDuration null))
  (set `self.TheHumanDescription` _returnvalue)
  (set `self.HumanDescriptionHidden?` true)
  (goto _label))

(event `/Game/Essential/PCToPawn_I.SpawnPackageInfos_I`
  (params (ColisType :type String) (De :type String))
  (bind _returnvalue (`|SpawnActorFromClass` "/Game/Blueprints/UserInterface/PackageDescription_BP.PackageDescription_BP_C" (`SceneComponent.K2_GetComponentToWorld` (`self.PlaceToSpawnHumanDescription`)) "Undefined" "OverrideRootScale" null ColisType De null))
  (set `self.ThePackageDescription` _returnvalue)
  (set `self.PackageDescriptionHidden` true)
  (goto _label_3))

(event `/Game/Essential/PCToPawn_I.DestroyPackageDescription_I`
  (bind _thepackagedescription (`self.ThePackageDescription`))
  (`/Engine/EditorBlueprintResources/StandardMacros.IsValid` _thepackagedescription
    (:`Is Valid`
      (`self.K2_DestroyActor` _thepackagedescription))))

(event `/Game/Essential/PCToPawn_I.DestroyPaperPackage_I`
  (`self.DestroyPaperPackage`))

(event `/Game/Essential/PCToPawn_I.DestroyHumanDescription_I`
  (bind _thehumandescription (`self.TheHumanDescription`))
  (`/Engine/EditorBlueprintResources/StandardMacros.IsValid` _thehumandescription
    (:`Is Valid`
      (`self.K2_DestroyActor` _thehumandescription))))

(event `/Game/Essential/PCToPawn_I.SpawnPaperHuman_I`
  (params (TheHuman :type "/Game/Blueprints/AI/HumanParent_BP Object Reference"))
  (`self.SpawnPaperHuman` TheHuman))

(event `/Game/Essential/PCToPawn_I.DestroyPaperHuman_I`
  (`self.DestroyPaperHuman`))

(event `/Game/Essential/PCToPawn_I.SpawnPaperPackage_I`
  (params (Box :type "/Game/Blueprints/ConvoyerBelt/BoxParent Object Reference"))
  (`self.SpawnPaperPackage` Box))

(fn `DestroyPaperHuman`
  (bind _tabofpaperhuman (`self.TabOfPaperHuman`))
  (for _array_element _tabofpaperhuman
    (`self.K2_DestroyActor` _array_element))
  (`KismetArrayLibrary.Array_Clear` _tabofpaperhuman)
  (`KismetArrayLibrary.Array_Clear` (`self.HumanPaperToSpawn`)))

(fn `DestroyPaperPackage`
  (bind _tabofpaperpackage (`self.TabOfPaperPackage`))
  (for _array_element _tabofpaperpackage
    (`self.K2_DestroyActor` _array_element))
  (`KismetArrayLibrary.Array_Clear` _tabofpaperpackage)
  (`KismetArrayLibrary.Array_Clear` (`self.PackagePaperToSpawn`)))

(fn `HandleDifficultyMode`
  (params (TheDifficulty :type "/Game/Essential/Difficulty_Enum Enum" :default "NewEnumerator0"))
  (switch `/Game/Essential/Difficulty_Enum` TheDifficulty
    (:`NewEnumerator0`
      (`TimelineComponent.SetPlayRate` (`self.DicreaseJaugePackage`) 0.0)
      (`TimelineComponent.SetPlayRate` (`self.DicreaseJaugeHuman`) 0.0)
      (set `self.FactorForBarPlus` 10.0)
      (set `self.FactorForBarMinus` 5.0))
    (:`NewEnumerator1`
      (`TimelineComponent.SetPlayRate` (`self.DicreaseJaugePackage`) 1.0)
      (`TimelineComponent.SetPlayRate` (`self.DicreaseJaugeHuman`) 1.0)
      (set `self.FactorForBarPlus` 10.0)
      (set `self.FactorForBarMinus` 5.0))
    (:`NewEnumerator2`
      (`TimelineComponent.SetPlayRate` (`self.DicreaseJaugePackage`) 2.0)
      (`TimelineComponent.SetPlayRate` (`self.DicreaseJaugeHuman`) 2.0)
      (set `self.FactorForBarPlus` 10.0)
      (set `self.FactorForBarMinus` 10.0))
    (:`NewEnumerator3`
      (`TimelineComponent.SetPlayRate` (`self.DicreaseJaugePackage`) 3.0)
      (`TimelineComponent.SetPlayRate` (`self.DicreaseJaugeHuman`) 3.0)
      (set `self.FactorForBarPlus` 5.0)
      (set `self.FactorForBarMinus` 10.0))))

(fn `SpawnPaperHuman`
  (params (TheHuman :type "/Game/Blueprints/AI/HumanParent_BP Object Reference"))
  (bind (_haveid _havepp _havecs _havevisaw _havevisas _havevisat _haveaptitude _havepermis _haveassurance _havepermistravail _havediplome) (`/Game/Blueprints/AI/HumanParent_BP.GiveHumanParams` TheHuman))
  (bind _humanpapertospawn (`self.HumanPaperToSpawn`))
  (bind (_returnvalue_roll _returnvalue_pitch) (`KismetMathLibrary.BreakRotator` (`SceneComponent.K2_GetComponentRotation` (`self.Camera`))))
  (if _haveid
    (`KismetArrayLibrary.Array_AddUnique` _humanpapertospawn "/Game/Blueprints/Papers/Human/CarteDIdentite_BP.CarteDIdentite_BP_C"))
  (if _havepp
    (`KismetArrayLibrary.Array_AddUnique` _humanpapertospawn "/Game/Blueprints/Papers/Human/PassePort_BP.PassePort_BP_C"))
  (if _havecs
    (`KismetArrayLibrary.Array_AddUnique` _humanpapertospawn "/Game/Blueprints/Papers/Human/PapierCitoyennete_BP.PapierCitoyennete_BP_C"))
  (if _havevisaw
    (`KismetArrayLibrary.Array_AddUnique` _humanpapertospawn "/Game/Blueprints/Papers/Human/VisaTravail_BP.VisaTravail_BP_C"))
  (if _havevisas
    (`KismetArrayLibrary.Array_AddUnique` _humanpapertospawn "/Game/Blueprints/Papers/Human/VisaEtude_BP.VisaEtude_BP_C"))
  (if _havevisat
    (`KismetArrayLibrary.Array_AddUnique` _humanpapertospawn "/Game/Blueprints/Papers/Human/VisaVoyage_BP.VisaVoyage_BP_C"))
  (if _haveaptitude
    (`KismetArrayLibrary.Array_AddUnique` _humanpapertospawn "/Game/Blueprints/Papers/Human/CertificatDAptitude_BP.CertificatDAptitude_BP_C"))
  (if _havepermis
    (`KismetArrayLibrary.Array_AddUnique` _humanpapertospawn "/Game/Blueprints/Papers/Human/PermisDeSejour_BP.PermisDeSejour_BP_C"))
  (if _haveassurance
    (`KismetArrayLibrary.Array_AddUnique` _humanpapertospawn "/Game/Blueprints/Papers/Human/AttestationDAssurance_BP.AttestationDAssurance_BP_C"))
  (if _havepermistravail
    (`KismetArrayLibrary.Array_AddUnique` _humanpapertospawn "/Game/Blueprints/Papers/Human/PermisDeTravail_BP.PermisDeTravail_BP_C"))
  (if _havediplome
    (`KismetArrayLibrary.Array_AddUnique` _humanpapertospawn "/Game/Blueprints/Papers/Human/DiplomeDAptitude_BP.DiplomeDAptitude_BP_C"))
  (for (_array_element _array_index) (`self.HumanPaperToSpawn`)
    (bind (_returnvalue_x _returnvalue_y _returnvalue_z) (`KismetMathLibrary.BreakVector` (`SceneComponent.K2_GetComponentLocation` (select `bool` (>= _array_index 3) :`false` (`self.PlaceToSpawnHumanPapersTop`) :`true` (`self.PlaceToSpawnHumanPapersDown`)))))
    (bind _returnvalue (`|SpawnActorFromClass` _array_element (`KismetMathLibrary.MakeTransform` (`KismetMathLibrary.MakeVector` (+ (* (mod (`KismetMathLibrary.Conv_IntToDouble` _array_index) 3.0) 10.0) _returnvalue_x) _returnvalue_y _returnvalue_z) (`KismetMathLibrary.MakeRotator` (+ _returnvalue_pitch 90.0) (`KismetMathLibrary.RandomFloatInRange` -5.0 5.0)) (0.9 1.0 0.8)) "Undefined" "OverrideRootScale" self null))
    (`KismetArrayLibrary.Array_AddUnique` (`self.TabOfPaperHuman`) _returnvalue)))

(fn `SpawnPaperPackage`
  (params (TheBox :type "/Game/Blueprints/ConvoyerBelt/BoxParent Object Reference"))
  (bind (_haveetiquette _haveattestationacquittement _haveeori _havepasseportanimal _havedae _havespecialautorisation _haveeurmed _havevaccination _havecertifmedical _havesps) (`/Game/Blueprints/ConvoyerBelt/BoxParent.GetPapers` TheBox))
  (bind _packagepapertospawn (`self.PackagePaperToSpawn`))
  (bind (_returnvalue_roll _returnvalue_pitch) (`KismetMathLibrary.BreakRotator` (`SceneComponent.K2_GetComponentRotation` (`self.Camera`))))
  (if _haveetiquette
    (`KismetArrayLibrary.Array_AddUnique` _packagepapertospawn "/Game/Blueprints/Papers/Box/Etiquette_BP.Etiquette_BP_C"))
  (if _haveattestationacquittement
    (`KismetArrayLibrary.Array_AddUnique` _packagepapertospawn "/Game/Blueprints/Papers/Box/AttestationDAcquittement_BP.AttestationDAcquittement_BP_C"))
  (if _haveeori
    (`KismetArrayLibrary.Array_AddUnique` _packagepapertospawn "/Game/Blueprints/Papers/Box/NuméroEORI_BP.NuméroEORI_BP_C"))
  (if _havepasseportanimal
    (`KismetArrayLibrary.Array_AddUnique` _packagepapertospawn "/Game/Blueprints/Papers/Box/PassePortAnimal_BP.PassePortAnimal_BP_C"))
  (if _havedae
    (`KismetArrayLibrary.Array_AddUnique` _packagepapertospawn "/Game/Blueprints/Papers/Box/DocumentDAccompegnementElectronique_BP.DocumentDAccompegnementElectronique_BP_C"))
  (if _havespecialautorisation
    (`KismetArrayLibrary.Array_AddUnique` _packagepapertospawn "/Game/Blueprints/Papers/Box/AutorisationSpeciale_BP.AutorisationSpeciale_BP_C"))
  (if _haveeurmed
    (`KismetArrayLibrary.Array_AddUnique` _packagepapertospawn "/Game/Blueprints/Papers/Box/CertificatEURMED_BP.CertificatEURMED_BP_C"))
  (if _havevaccination
    (`KismetArrayLibrary.Array_AddUnique` _packagepapertospawn "/Game/Blueprints/Papers/Box/CertificatVaccination_BP.CertificatVaccination_BP_C"))
  (if _havecertifmedical
    (`KismetArrayLibrary.Array_AddUnique` _packagepapertospawn "/Game/Blueprints/Papers/Box/CertificatMedical_BP.CertificatMedical_BP_C"))
  (if _havesps
    (`KismetArrayLibrary.Array_AddUnique` _packagepapertospawn "/Game/Blueprints/Papers/Box/SPS_BP.SPS_BP_C"))
  (for (_array_element _array_index) (`self.PackagePaperToSpawn`)
    (bind (_returnvalue_x _returnvalue_y _returnvalue_z) (`KismetMathLibrary.BreakVector` (`SceneComponent.K2_GetComponentLocation` (select `bool` (>= _array_index 3) :`false` (`self.PlaceToSpawnPackagesPapersTop`) :`true` (`self.PlaceToSpawnPackagesPapersDown`)))))
    (bind _returnvalue (`|SpawnActorFromClass` _array_element (`KismetMathLibrary.MakeTransform` (`KismetMathLibrary.MakeVector` (+ (* (mod (`KismetMathLibrary.Conv_IntToDouble` _array_index) 3.0) 10.0) _returnvalue_x) _returnvalue_y _returnvalue_z) (`KismetMathLibrary.MakeRotator` (+ _returnvalue_pitch 90.0) (`KismetMathLibrary.RandomFloatInRange` -5.0 5.0)) (0.9 1.0 0.8)) "Undefined" "OverrideRootScale" self null))
    (`KismetArrayLibrary.Array_AddUnique` (`self.TabOfPaperPackage`) _returnvalue)))

(fn `UserConstructionScript`)