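; Tutorial spawner that runs the queue of travelers at the passport desk and applies the player's accept or reject.
; Construction lays out line slots behind the desk trigger; SpawnPeople spawns a human flagged good or bad at the last slot.
; Reaching the desk shows their paper and info through the tutorial camera pawn.
; Yes sends them on, No launches them with a spring; both update gauges and advance the line.
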(event `self.ReceiveBeginPlay`
  ;[1 1 1] Begin play
  (bind _asthe_player_camera_for_tuto_bp (cast `/Game/Level/TutoGuideMap/ThePlayerCameraForTuto_BP` (`GameplayStatics.GetPlayerPawn` 0)))
  (bind _output_get (set `self.ThePlayer` _asthe_player_camera_for_tuto_bp))
  (set `/Game/Level/TutoGuideMap/ThePlayerCameraForTuto_BP.TheHuman` self _output_get)
  (bind _asspring_bp (cast `/Game/Blueprints/Spring/Spring_Bp` (`ChildActorComponent.ChildActor` (`self.Spring`))))
  (set `self.MySpring` _asspring_bp))

(event `self.BoxEnd.OnComponentBeginOverlap`
  (params (OverlappedComponent :type "PrimitiveComponent Object Reference") (OtherActor :type "Actor Object Reference") (OtherComp :type "PrimitiveComponent Object Reference") (OtherBodyIndex :type Integer) (bFromSweep :type Boolean) (SweepResult :type "HitResult Structure (by ref)"))
  (bind _theplayer (`self.ThePlayer`))
  ;[1 1 1] Tend le passport quand il est proche du bureau
  (if (!= OtherActor (`self.TheHuman`))
    (bind _ashuman_parent_bp (cast `/Game/Blueprints/AI/Humans/HumanParent_BP` OtherActor))
    (bind _output_get (set `self.TheHuman` _ashuman_parent_bp))
    (`/Game/Level/TutoGuideMap/ThePlayerCameraForTuto_BP.SpawnPaperHuman` _theplayer _output_get)
    (`/Game/Level/TutoGuideMap/ThePlayerCameraForTuto_BP.SpawnHumanInfos` _theplayer (`/Game/Blueprints/AI/Humans/HumanParent_BP.Prenom` _output_get) (`/Game/Blueprints/AI/Humans/HumanParent_BP.TravelType` _output_get) (`/Game/Blueprints/AI/Humans/HumanParent_BP.Duration` _output_get))
    (`/Game/Blueprints/AI/Humans/HumanParent_BP.SetisGiving` _output_get)
    (`/Engine/EditorBlueprintResources/StandardMacros.DoOnce` false
      (:`Completed`
        (`/Game/Level/TutoGuideMap/ThePlayerCameraForTuto_BP.BaisseJaugeHuman` (`self.ThePlayer`))))))

(event `SpawnPeople`
  (params (goodPeople :type Boolean))
  (bind _targetpoints (`self.TargetPoints`))
  (bind _targetpointsoccuped (`self.TargetPointsOccuped`))
  ;[1 1 1] Spawn un personnage aléatoire en fonction d'un temps aléatoire
  (bind _returnvalue (`AIBlueprintHelperLibrary.SpawnAIFromClass` "/Game/Level/TutoGuideMap/HumanParentForTuto_BP.HumanParentForTuto_BP_C" null (`KismetMathLibrary.TransformLocation` (`self.GetTransform`) (`|GetArrayItem` _targetpoints (`KismetArrayLibrary.Array_LastIndex` _targetpoints))) (struct :`Yaw` 90.0) true))
  (bind _ashuman_parent_bp (cast `/Game/Blueprints/AI/Humans/HumanParent_BP` _returnvalue))
  (set `/Game/Blueprints/AI/Humans/HumanParent_BP.IsAGoodHuman` goodPeople _ashuman_parent_bp)
  (`KismetArrayLibrary.Array_Add` (`self.MyHumanArray`) _ashuman_parent_bp)
  (`KismetArrayLibrary.Array_Set` _targetpointsoccuped (`KismetArrayLibrary.Array_LastIndex` _targetpointsoccuped) true)
  (`/Game/Blueprints/AI/Humans/HumanParent_BP.Move` _ashuman_parent_bp false))

(event `self.BoxForDestroy.OnComponentBeginOverlap`
  (params (OverlappedComponent :type "PrimitiveComponent Object Reference") (OtherActor :type "Actor Object Reference") (OtherComp :type "PrimitiveComponent Object Reference") (OtherBodyIndex :type Integer) (bFromSweep :type Boolean) (SweepResult :type "HitResult Structure (by ref)"))
  (`self.K2_DestroyActor` OtherActor))

(fn `No`
  (bind _theplayer (`self.ThePlayer`))
  (bind _thehuman (`self.TheHuman`))
  (`/Game/Level/TutoGuideMap/ThePlayerCameraForTuto_BP.DestroyPaperHuman` _theplayer)
  (`/Game/Level/TutoGuideMap/ThePlayerCameraForTuto_BP.DestroyHumanDescription` _theplayer)
  (`/Engine/EditorBlueprintResources/StandardMacros.IsValid` _thehuman
    (:`Is Valid`
      (`/Game/Level/TutoGuideMap/ThePlayerCameraForTuto_BP.ChangeJaugesHuman` (`self.ThePlayer`) (`/Game/Blueprints/AI/Humans/HumanParent_BP.IsAGoodHuman` _thehuman))
      (`/Game/Blueprints/Spring/Spring_Bp.Boing` (`self.MySpring`))
      (`Character.LaunchCharacter` _thehuman (0.0 0.0 1000.0) false false)
      (`KismetArrayLibrary.Array_Set` (`self.TargetPointsOccuped`))
      (for _array_element (`self.MyHumanArray`)
        (`/Engine/EditorBlueprintResources/StandardMacros.IsValid` _array_element
          (:`Is Valid`
            (`/Game/Blueprints/AI/Humans/HumanParent_BP.Move` _array_element false)))))))

(fn `UserConstructionScript`
  (bind (_relativelocation_x _relativelocation_y _relativelocation_z) (`KismetMathLibrary.BreakVector` (`SceneComponent.RelativeLocation` (`self.BoxEnd`))))
  (`KismetArrayLibrary.Array_Clear` (`self.TargetPoints`))
  (`KismetArrayLibrary.Array_Clear` (`self.TargetPointsOccuped`))
  (for _index (range (+ (`self.NumberOfPeopleInLine`) 1))
    (`KismetArrayLibrary.Array_Add` (`self.TargetPoints`) (`KismetMathLibrary.MakeVector` _relativelocation_x (- _relativelocation_y (`KismetMathLibrary.Conv_IntToDouble` (* _index (`self.DistanceFromPeopleToPeople`)))) (+ _relativelocation_z 100.0)))
    (`KismetArrayLibrary.Array_Add` (`self.TargetPointsOccuped`))))

(fn `Yes`
  (bind _theplayer (`self.ThePlayer`))
  (bind _thehuman (`self.TheHuman`))
  (`/Game/Level/TutoGuideMap/ThePlayerCameraForTuto_BP.DestroyPaperHuman` _theplayer)
  (`/Game/Level/TutoGuideMap/ThePlayerCameraForTuto_BP.DestroyHumanDescription` _theplayer)
  (`/Engine/EditorBlueprintResources/StandardMacros.IsValid` _thehuman
    (:`Is Valid`
      (`/Game/Level/TutoGuideMap/ThePlayerCameraForTuto_BP.ChangeJaugesHuman` (`self.ThePlayer`) (not (`/Game/Blueprints/AI/Humans/HumanParent_BP.IsAGoodHuman` _thehuman)))
      (`/Game/Blueprints/AI/Humans/HumanParent_BP.Move` _thehuman true)
      (`KismetArrayLibrary.Array_Set` (`self.TargetPointsOccuped`))
      (for _array_element (`self.MyHumanArray`)
        (`/Engine/EditorBlueprintResources/StandardMacros.IsValid` _array_element
          (:`Is Valid`
            (`/Game/Blueprints/AI/Humans/HumanParent_BP.Move` _array_element false)))))))