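; Tutorial human spawner that runs a passport-check queue, registering itself with the tutorial PlayerController.
; The construction script lays out queue points back from the desk; SpawnPeople spawns a good or bad AI human at the last one.
; Reaching BoxEnd shows papers and info through pawn interface messages and notifies the controller.
; Yes walks the human on, No spring-launches them; both update the gauge and advance the line, while destroy boxes remove overlapping actors.
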(event `self.ReceiveBeginPlay`
  ;[1 1 1] Begin play
  (bind _asmy_player_controller_tuto (cast `/Game/Level/TutoGuideMap/Essential/MyPlayerControllerTuto` (`GameplayStatics.GetPlayerController` 0)))
  (bind _output_get (set `self.PlayerController` _asmy_player_controller_tuto))
  (set `/Game/Level/TutoGuideMap/Essential/MyPlayerControllerTuto.TheHuman` self _output_get)
  (bind _asspring_bp (cast `/Game/Blueprints/Spring/Spring_Bp` (`ChildActorComponent.ChildActor` (`self.Spring`))))
  (set `self.MySpring` _asspring_bp))

(event `self.BoxEnd.OnComponentBeginOverlap`
  (params (OverlappedComponent :type "PrimitiveComponent Object Reference") (OtherActor :type "Actor Object Reference") (OtherComp :type "PrimitiveComponent Object Reference") (OtherBodyIndex :type Integer) (bFromSweep :type Boolean) (SweepResult :type "HitResult Structure (by ref)"))
  (bind _returnvalue (`GameplayStatics.GetPlayerPawn` 0))
  ;[1 1 1] Tend le passport quand il est proche du bureau
  (bind _ashuman_parent_for_tuto_bp (cast `/Game/Level/TutoGuideMap/BluePrint/HumanParentForTuto_BP` OtherActor))
  (bind _output_get (set `self.TheHuman` _ashuman_parent_for_tuto_bp))
  (message `/Game/Level/TutoGuideMap/Essential/PCToPawnForTuto_I.SpawnPaperHuman_I` _returnvalue _output_get)
  (message `/Game/Level/TutoGuideMap/Essential/PCToPawnForTuto_I.SpawnHumanInfo_I` _returnvalue (`/Game/Level/TutoGuideMap/BluePrint/HumanParentForTuto_BP.Prenom` _output_get) (`/Game/Level/TutoGuideMap/BluePrint/HumanParentForTuto_BP.TravelType` _output_get) (`/Game/Level/TutoGuideMap/BluePrint/HumanParentForTuto_BP.Duration` _output_get))
  (`/Game/Level/TutoGuideMap/BluePrint/HumanParentForTuto_BP.SetIsGiving` _output_get)
  (`/Game/Level/TutoGuideMap/Essential/MyPlayerControllerTuto.EventHumanArrived` (`self.PlayerController`)))

(event `SpawnPeople`
  (params (GoodHuman :type Boolean))
  (bind _targetpoints (`self.TargetPoints`))
  ;[1 1 1] Spawn un personnage aléatoire en fonction d'un temps aléatoire
  (bind _returnvalue (`AIBlueprintHelperLibrary.SpawnAIFromClass` "/Game/Level/TutoGuideMap/BluePrint/HumanParentForTuto_BP.HumanParentForTuto_BP_C" null (`KismetMathLibrary.TransformLocation` (`self.GetTransform`) (`|GetArrayItem` _targetpoints (`KismetArrayLibrary.Array_LastIndex` _targetpoints))) (struct :`Yaw` 90.0) true))
  (bind _ashuman_parent_for_tuto_bp (cast `/Game/Level/TutoGuideMap/BluePrint/HumanParentForTuto_BP` _returnvalue))
  (set `/Game/Level/TutoGuideMap/BluePrint/HumanParentForTuto_BP.ShouldSpawnAGoodGuy` GoodHuman _ashuman_parent_for_tuto_bp)
  (`KismetArrayLibrary.Array_Add` (`self.MyHumanArray`) _ashuman_parent_for_tuto_bp)
  (`/Game/Level/TutoGuideMap/BluePrint/HumanParentForTuto_BP.Move` _ashuman_parent_for_tuto_bp false))

(event `self.BoxForDestroy.OnComponentBeginOverlap`
  (params (OverlappedComponent :type "PrimitiveComponent Object Reference") (OtherActor :type "Actor Object Reference") (OtherComp :type "PrimitiveComponent Object Reference") (OtherBodyIndex :type Integer) (bFromSweep :type Boolean) (SweepResult :type "HitResult Structure (by ref)"))
  (`self.K2_DestroyActor` OtherActor)
  (`KismetArrayLibrary.Array_Set` (`self.TargetPointsOccuped`) :!label _label))

(event `self.BoxForDestroy1.OnComponentBeginOverlap`
  (params (OverlappedComponent :type "PrimitiveComponent Object Reference") (OtherActor :type "Actor Object Reference") (OtherComp :type "PrimitiveComponent Object Reference") (OtherBodyIndex :type Integer) (bFromSweep :type Boolean) (SweepResult :type "HitResult Structure (by ref)"))
  (`self.K2_DestroyActor` OtherActor)
  (goto _label))

(fn `No`
  (bind _returnvalue (`GameplayStatics.GetPlayerPawn` 0))
  (bind _thehuman (`self.TheHuman`))
  (`|ExecutionSequence`
    (:`then_0`
      (message `/Game/Level/TutoGuideMap/Essential/PCToPawnForTuto_I.DestroyPaperPackage_I` _returnvalue)
      (message `/Game/Level/TutoGuideMap/Essential/PCToPawnForTuto_I.DestroyHumanDescription_I` _returnvalue)
      (`/Engine/EditorBlueprintResources/StandardMacros.IsValid` _thehuman
        (:`Is Valid`
          (message `/Game/Level/TutoGuideMap/Essential/PCToPawnForTuto_I.ChangeJaugeHuman_I` (`GameplayStatics.GetPlayerPawn` 0) (`/Game/Level/TutoGuideMap/BluePrint/HumanParentForTuto_BP.IsAGoodHuman` _thehuman))
          (`/Game/Blueprints/Spring/Spring_Bp.Boing` (`self.MySpring`))
          (`Character.LaunchCharacter` _thehuman (0.0 0.0 1000.0) false false))))
    (:`then_1`
      (`KismetArrayLibrary.Array_Set` (`self.TargetPointsOccuped`))
      (for _array_element (`self.MyHumanArray`)
        (`/Engine/EditorBlueprintResources/StandardMacros.IsValid` _array_element
          (:`Is Valid`
            (`/Game/Level/TutoGuideMap/BluePrint/HumanParentForTuto_BP.Move` _array_element false)))))))

(fn `UserConstructionScript`
  (bind (_relativelocation_x _relativelocation_y _relativelocation_z) (`KismetMathLibrary.BreakVector` (`SceneComponent.RelativeLocation` (`self.BoxEnd`))))
  (`KismetArrayLibrary.Array_Clear` (`self.TargetPoints`))
  (`KismetArrayLibrary.Array_Clear` (`self.TargetPointsOccuped`))
  (for _index (range (+ (`self.NumberOfPeopleInLine`) 1))
    (`KismetArrayLibrary.Array_Add` (`self.TargetPoints`) (`KismetMathLibrary.MakeVector` _relativelocation_x (- _relativelocation_y (`KismetMathLibrary.Conv_IntToDouble` (* _index (`self.DistanceFromPeopleToPeople`)))) (+ _relativelocation_z 100.0)))
    (`KismetArrayLibrary.Array_Add` (`self.TargetPointsOccuped`))))

(fn `Yes`
  (bind _returnvalue (`GameplayStatics.GetPlayerPawn` 0))
  (bind _thehuman (`self.TheHuman`))
  (`|ExecutionSequence`
    (:`then_0`
      (message `/Game/Level/TutoGuideMap/Essential/PCToPawnForTuto_I.DestroyPaperPackage_I` _returnvalue)
      (message `/Game/Level/TutoGuideMap/Essential/PCToPawnForTuto_I.DestroyHumanDescription_I` _returnvalue)
      (`/Engine/EditorBlueprintResources/StandardMacros.IsValid` _thehuman
        (:`Is Valid`
          (message `/Game/Level/TutoGuideMap/Essential/PCToPawnForTuto_I.ChangeJaugeHuman_I` (`GameplayStatics.GetPlayerPawn` 0) (not (`/Game/Level/TutoGuideMap/BluePrint/HumanParentForTuto_BP.IsAGoodHuman` _thehuman)))
          (`/Game/Level/TutoGuideMap/BluePrint/HumanParentForTuto_BP.Move` _thehuman true))))
    (:`then_1`
      (`KismetArrayLibrary.Array_Set` (`self.TargetPointsOccuped`))
      (for _array_element (`self.MyHumanArray`)
        (`/Engine/EditorBlueprintResources/StandardMacros.IsValid` _array_element
          (:`Is Valid`
            (`/Game/Level/TutoGuideMap/BluePrint/HumanParentForTuto_BP.Move` _array_element false)))))))