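; Pause control for the tutorial guide map that freezes the game when clicked.
; On BeginPlay it registers itself as ThePause on the tutorial player controller, MyPlayerControllerTuto.
; When Clicked fires and IsClickable is true, it pauses the game and calls SetPause on MyHUDTuto.
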(event `self.ReceiveBeginPlay`
  (bind _asmy_player_controller_tuto (cast `/Game/Level/TutoGuideMap/Essential/MyPlayerControllerTuto` (`GameplayStatics.GetPlayerController` 0)))
  (set `/Game/Level/TutoGuideMap/Essential/MyPlayerControllerTuto.ThePause` self _asmy_player_controller_tuto))

(event `/Game/Blueprints/ClickedEvent.Clicked`
  (params (Component :type "ActorComponent Object Reference"))
  (if (`self.IsClickable`)
    (`GameplayStatics.SetGamePaused` true)
    (bind _asmy_hudtuto (cast `/Game/Level/TutoGuideMap/Essential/MyHUDTuto` (`PlayerController.GetHUD` (`GameplayStatics.GetPlayerController` 0))))
    (`/Game/Level/TutoGuideMap/Essential/MyHUDTuto.SetPause` _asmy_hudtuto)))

(fn `UserConstructionScript`)