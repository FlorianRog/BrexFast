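; Parent Blueprint for tutorial package boxes, each with a random size, sender (company or individual) and content type drawn from the BD_PackageType data table.
; BeginPlay copies the row's category flags, swaps the mesh for pets, and sets the label and good-box flags from ShouldBeGoodBox.
; GetPapers exposes the label flag.
; After touching the tutorial conveyor belt, a box destroys other boxes that overlap its Boite component.
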(event `self.Boite.OnComponentBeginOverlap`
  (params (OverlappedComponent :type "PrimitiveComponent Object Reference") (OtherActor :type "Actor Object Reference") (OtherComp :type "PrimitiveComponent Object Reference") (OtherBodyIndex :type Integer) (bFromSweep :type Boolean) (SweepResult :type "HitResult Structure (by ref)"))
  (if (!= OtherActor self)
    (cast `/Game/Level/TutoGuideMap/BluePrint/ConvoyerBeltForTuto_BP` OtherActor
      (:`then`
        (set `self.CanDestroy` true))
      (:`CastFailed`
        (cast `/Game/Level/TutoGuideMap/BluePrint/BoxParentForTuto_BP` OtherActor)
        (if (`self.CanDestroy`)
          (`self.K2_DestroyActor` OtherActor))))))

(event `self.ReceiveBeginPlay`
  (if (`KismetMathLibrary.RandomBool`)
    (set `self.Entreprise?` true)
    (set `self.From` "Entreprise")
    (else
      (set `self.Particulier?` true)
      (set `self.From` "Particulier")))
  (bind _outrownames (`DataTableFunctionLibrary.GetDataTableRowNames` "/Game/Blueprints/Databases/Packages/BD_PackageType.BD_PackageType"))
  (set `self.RandomPackageType` (`KismetMathLibrary.RandomIntegerInRange` 0 (- (`KismetArrayLibrary.Array_Length` _outrownames) 1)))
  (for (_array_element _array_index) _outrownames
    (if (== _array_index (`self.RandomPackageType`))
      (bind _returnvalue (`|GetDataTableRow` "/Game/Blueprints/Databases/Packages/BD_PackageType.BD_PackageType" _array_element)
        (:`then`
          (bind (_packagetype _ispet _isdangerous _isstup _isother) (break `/Game/Blueprints/Databases/Packages/STDT_PackageType` _returnvalue))
          (set `self.PackageType` _packagetype)
          (set `self.IsAPet` _ispet)
          (set `self.IsDangerous` _isdangerous)
          (set `self.IsStup` _isstup)
          (set `self.IsOther` _isother)))))
  ;[1 1 1] Change the box
  (if (`self.IsAPet`)
    (`StaticMeshComponent.SetStaticMesh` (`self.TheBox`) "/Game/Assets/StaticMeshes/varisalacanelle.varisalacanelle"))
  ;[1 1 1] CheckEtiquette
  (bind _output_get (set `self.HaveEtiquette` (`self.ShouldBeGoodBox`)))
  (set `self.IsAGoodBox` _output_get))

(fn `GetPapers`
  (returns (HaveEtiquette :type Boolean))
  (return (`self.HaveEtiquette`)))

(fn `UserConstructionScript`
  (bind _boite (`self.Boite`))
  (`self.SetActorScale3D` (`KismetMathLibrary.MakeVector` (`KismetMathLibrary.RandomFloatInRange` 0.5 1.5) (`KismetMathLibrary.RandomFloatInRange` 0.5 1.5) (`KismetMathLibrary.RandomFloatInRange` 0.5 1.5)))
  (`SceneComponent.SetRelativeScale3D` _boite (* (`SceneComponent.RelativeScale3D` _boite) 1.6)))