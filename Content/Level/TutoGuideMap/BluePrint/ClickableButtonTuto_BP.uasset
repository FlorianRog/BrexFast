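; ClickableButtonTuto_BP is a clickable mesh button in the tutorial guide map that gives a Yes or No answer for either the human or the package (carpet).
; The IsYes and IsHuman flags choose its check or cross material in the Construction Script.
; On click, if clickable, it calls Yes or No on the tutorial player controller's human or carpet, fires that controller's matching button event, then disables further clicks.
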(event `self.ReceiveBeginPlay`
  (bind _asmy_player_controller_tuto (cast `/Game/Level/TutoGuideMap/Essential/MyPlayerControllerTuto` (`GameplayStatics.GetPlayerController` 0)))
  (set `self.ThePlayer` _asmy_player_controller_tuto))

(event `/Game/Blueprints/ClickedEvent.Clicked`
  (params (Component :type "ActorComponent Object Reference"))
  (bind _theplayer (`self.ThePlayer`))
  (bind _thecarpet (`/Game/Level/TutoGuideMap/Essential/MyPlayerControllerTuto.TheCarpet` (`self.ThePlayer`)))
  (bind _thehuman (`/Game/Level/TutoGuideMap/Essential/MyPlayerControllerTuto.TheHuman` (`self.ThePlayer`)))
  (if (`self.IsClickable`)
    (if (`self.IsHuman`)
      (if (`self.IsYes`)
        (`/Game/Level/TutoGuideMap/BluePrint/HumanSpawnerForTuto_BP.Yes` _thehuman)
        (`/Game/Level/TutoGuideMap/Essential/MyPlayerControllerTuto.EventBTNYesHumanClicked` _theplayer)
        (else
          (`/Game/Level/TutoGuideMap/BluePrint/HumanSpawnerForTuto_BP.No` _thehuman)
          (`/Game/Level/TutoGuideMap/Essential/MyPlayerControllerTuto.EventBTNNoHumanClicked` _theplayer)))
      (elif (`self.IsYes`)
        (`/Game/Level/TutoGuideMap/BluePrint/ConvoyerBeltForTuto_BP.Yes` _thecarpet)
        (`/Game/Level/TutoGuideMap/Essential/MyPlayerControllerTuto.EventBTNYesPackageClicked` _theplayer)
        (else
          (`/Game/Level/TutoGuideMap/BluePrint/ConvoyerBeltForTuto_BP.No` _thecarpet)
          (`/Game/Level/TutoGuideMap/Essential/MyPlayerControllerTuto.EventBTNNoPackageClicked` _theplayer))))
    (set `self.IsClickable` false)))

(fn `UserConstructionScript`
  (bind _staticmesh (`self.StaticMesh`))
  (bind _staticmesh_2 (`self.StaticMesh`))
  (if (`self.IsYes`)
    (if (`self.IsHuman`)
      (`PrimitiveComponent.SetMaterial` _staticmesh_2 0 "/Game/Assets/MaterialAndTextures/Materiaux/BaseTexture/Childs/BT_CheckHuman.BT_CheckHuman")
      (else
        (`PrimitiveComponent.SetMaterial` _staticmesh_2 0 "/Game/Assets/MaterialAndTextures/Materiaux/BaseTexture/Childs/BT_CheckPackage.BT_CheckPackage")))
    (elif (`self.IsHuman`)
      (`PrimitiveComponent.SetMaterial` _staticmesh 0 "/Game/Assets/MaterialAndTextures/Materiaux/BaseTexture/Childs/BT_CrossHuman.BT_CrossHuman")
      (else
        (`PrimitiveComponent.SetMaterial` _staticmesh 0 "/Game/Assets/MaterialAndTextures/Materiaux/BaseTexture/Childs/BT_CrossPackage.BT_CrossPackage")))))