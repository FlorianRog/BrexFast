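; Tutorial conveyor belt that carries packages to an inspection zone where the player accepts or rejects them.
; Tick slides boxes overlapping the movement volume until one enters the treatment zone, which centers it, stops the belt and shows its paperwork through pawn interface messages.
; Yes or No reports whether the choice was right to a gauge, launches the box (No also fires the spring) and restarts the belt.
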(event `self.ReceiveBeginPlay`
  ;[1 1 1] Set a few variables
  (bind _asmy_player_controller_tuto (cast `/Game/Level/TutoGuideMap/Essential/MyPlayerControllerTuto` (`GameplayStatics.GetPlayerController` 0)))
  (bind _output_get (set `self.ThePlayerController` _asmy_player_controller_tuto))
  (set `/Game/Level/TutoGuideMap/Essential/MyPlayerControllerTuto.TheCarpet` self _output_get)
  (set `self.TheDirection` (`self.NormalDirection`))
  (set `self.BoxForMovements` (`self.NormalMovementBox`))
  (bind _asspring_bp (cast `/Game/Blueprints/Spring/Spring_Bp` (`ChildActorComponent.ChildActor` (`self.Spring`))))
  (set `self.MySpring` _asspring_bp))

(event `self.ReceiveTick`
  (params (DeltaSeconds :type "Float (single-precision)"))
  ;[1 1 1] Adding movement to the convoyer belt
  (for _array_element (`PrimitiveComponent.GetOverlappingActors` (`self.BoxForMovements`) "/Game/Blueprints/ConvoyerBelt/BoxParent.BoxParent_C")
    (if (!= _array_element self)
      (`self.K2_AddActorWorldOffset` _array_element (* (`SceneComponent.GetForwardVector` (`self.TheDirection`)) (* DeltaSeconds (`self.Speed`))) false false))))

(event `SpawnBoxes`
  ;[1 1 1] spawn boxes
  (`|SpawnActorFromClass` "/Game/Blueprints/ConvoyerBelt/BoxParent.BoxParent_C" (`SceneComponent.K2_GetComponentToWorld` (`self.PlaceToSpawn`)) "Undefined" "OverrideRootScale" null null))

(event `self.InTraitment.OnComponentBeginOverlap`
  (params (OverlappedComponent :type "PrimitiveComponent Object Reference") (OtherActor :type "Actor Object Reference") (OtherComp :type "PrimitiveComponent Object Reference") (OtherBodyIndex :type Integer) (bFromSweep :type Boolean) (SweepResult :type "HitResult Structure (by ref)"))
  (bind _returnvalue (`GameplayStatics.GetPlayerPawn` 0))
  ;[1 1 1] On traitement box overlap, move the box to the center and disable the convoyer belt movement
  (if (!= OtherActor (`self.TheBox`))
    (bind _asbox_parent_for_tuto_bp (cast `/Game/Level/TutoGuideMap/BluePrint/BoxParentForTuto_BP` OtherActor))
    (set `self.CanSpawn` false)
    (bind _output_get (set `self.TheBox` _asbox_parent_for_tuto_bp))
    (`self.SetActorTickEnabled` false)
    (message `/Game/Level/TutoGuideMap/Essential/PCToPawnForTuto_I.SpawnPaperPackage_I` _returnvalue _output_get)
    (message `/Game/Essential/PCToPawn_I.SpawnPackageInfos_I` _returnvalue (`/Game/Level/TutoGuideMap/BluePrint/BoxParentForTuto_BP.PackageType` _output_get) (`/Game/Level/TutoGuideMap/BluePrint/BoxParentForTuto_BP.From` _output_get))
    (`KismetSystemLibrary.MoveComponentTo` (`Actor.RootComponent` _output_get) (`SceneComponent.K2_GetComponentLocation` (`self.InTraitment`)))
    (`/Engine/EditorBlueprintResources/StandardMacros.DoOnce` false
      (:`Completed`
        (message `/Game/Essential/PCToPawn_I.BaisseJaugePackage_I` (`GameplayStatics.GetPlayerPawn` 0))))))

(fn `No`
  (bind _returnvalue (`GameplayStatics.GetPlayerPawn` 0))
  (bind _thebox (`self.TheBox`))
  (message `/Game/Essential/PCToPawn_I.DestroyPaperPackage_I` _returnvalue)
  (message `/Game/Essential/PCToPawn_I.DestroyPackageDescription_I` _returnvalue)
  (`/Engine/EditorBlueprintResources/StandardMacros.IsValid` _thebox
    (:`Is Valid`
      (message `/Game/Essential/PCToPawn_I.ChangeJaugePackage_I` (`GameplayStatics.GetPlayerPawn` 0) (`/Game/Level/TutoGuideMap/BluePrint/BoxParentForTuto_BP.IsAGoodBox` _thebox))
      (`/Game/Blueprints/Spring/Spring_Bp.Boing` (`self.MySpring`))
      (`PrimitiveComponent.AddImpulse` (`/Game/Level/TutoGuideMap/BluePrint/BoxParentForTuto_BP.TheBox` (`self.TheBox`)) (0.0 0.0 5000000.0) "None" false)
      (`self.SetActorTickEnabled` true)
      (set `self.CanSpawn` true))))

(fn `UserConstructionScript`)

(fn `Yes`
  (bind _returnvalue (`GameplayStatics.GetPlayerPawn` 0))
  (bind _thebox (`self.TheBox`))
  (message `/Game/Essential/PCToPawn_I.DestroyPaperPackage_I` _returnvalue)
  (message `/Game/Essential/PCToPawn_I.DestroyPackageDescription_I` _returnvalue)
  (`/Engine/EditorBlueprintResources/StandardMacros.IsValid` _thebox
    (:`Is Valid`
      (message `/Game/Essential/PCToPawn_I.ChangeJaugePackage_I` (`GameplayStatics.GetPlayerPawn` 0) (not (`/Game/Level/TutoGuideMap/BluePrint/BoxParentForTuto_BP.IsAGoodBox` _thebox)))
      (`PrimitiveComponent.AddImpulse` (`/Game/Level/TutoGuideMap/BluePrint/BoxParentForTuto_BP.TheBox` (`self.TheBox`)) (-2500000.0 0.0 0.0) "None" false)
      (`self.SetActorTickEnabled` true)
      (set `self.CanSpawn` true))))