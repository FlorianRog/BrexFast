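; SlideBarTuto_BP is a world-space slide bar for the tutorial map that displays one of the player's two time values, human or package, chosen by IsHuman.
; BeginPlay caches the bar's initial X scale and the ThePlayerCameraForTuto_BP pawn.
; Each Tick maps the selected time to a clamped X scale on the bar.
; It also drives the material's Alpha parameter from how far the bar has shrunk relative to its initial scale.
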(event `self.ReceiveBeginPlay`
  (bind _returnvalue_x (`KismetMathLibrary.BreakVector` (`SceneComponent.K2_GetComponentScale` (`self.Bar`))))
  (set `self.InitlaXScale` _returnvalue_x)
  (bind _asthe_player_camera_for_tuto_bp (cast `/Game/Level/TutoGuideMap/Essential/ThePlayerCameraForTuto_BP` (`GameplayStatics.GetPlayerPawn` 0)))
  (set `self.ThePlayer` _asthe_player_camera_for_tuto_bp))

(event `self.ReceiveTick`
  (params (DeltaSeconds :type "Float (single-precision)"))
  (bind _theplayer (`self.ThePlayer`))
  (bind _bar (`self.Bar`))
  (bind _returnvalue_x (`KismetMathLibrary.BreakVector` (`SceneComponent.K2_GetComponentScale` _bar)))
  (bind (_returnvalue_x_2 _returnvalue_y _returnvalue_z) (`KismetMathLibrary.BreakVector` (`SceneComponent.K2_GetComponentScale` (`self.Bar`))))
  (`/Engine/EditorBlueprintResources/StandardMacros.IsValid` _theplayer
    (:`Is Valid`
      (if (`self.IsHuman`)
        (set `self.CurrentTime` (`/Game/Level/TutoGuideMap/Essential/ThePlayerCameraForTuto_BP.TimeHuman` _theplayer))
        (else
          (set `self.CurrentTime` (`/Game/Level/TutoGuideMap/Essential/ThePlayerCameraForTuto_BP.TimePackage` _theplayer))))
      (`SceneComponent.SetWorldScale3D` (`self.Bar`) (`KismetMathLibrary.MakeVector` (`KismetMathLibrary.FClamp` (/ (`self.CurrentTime`) 100.0)) _returnvalue_y _returnvalue_z))
      (`MeshComponent.SetScalarParameterValueOnMaterials` _bar "Alpha" (- 1.0 (/ _returnvalue_x (`self.InitlaXScale`)))))))

(fn `UserConstructionScript`)