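; HumanDescription_BP is a clickable description of a human traveler, showing a name, travel motive and journey duration.
; The construction script writes these variables into three text render components, adding French labels to the motive and duration.
; On click, it sends the PlayAnimationHumanDescription interface message to the player pawn, leaving any animation to that pawn's implementation.
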(event `self.ReceiveBeginPlay`)

(event `/Game/Blueprints/ClickedEvent.Clicked`
  (params (Component :type "ActorComponent Object Reference"))
  (message `/Game/Essential/PCToPawn_I.PlayAnimationHumanDescription_I` (`GameplayStatics.GetPlayerPawn` 0)))

(fn `UserConstructionScript`
  (`TextRenderComponent.K2_SetText` (`self.TextRender`) (`KismetTextLibrary.Conv_StringToText` (`self.Name`)))
  (`TextRenderComponent.K2_SetText` (`self.TextRender1`) (`KismetTextLibrary.Conv_StringToText` (`KismetStringLibrary.Concat_StrStr` "Motif : " (`self.TravelerType`))))
  (`TextRenderComponent.K2_SetText` (`self.TextRender2`) (`KismetTextLibrary.Conv_StringToText` (`KismetStringLibrary.Concat_StrStr` "Durée : " (`self.JourneyDuration`)))))