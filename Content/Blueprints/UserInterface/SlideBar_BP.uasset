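; SlideBar_BP is a world-space progress bar that displays one of two timer values from the player's ThePlayerCamera pawn.
; BeginPlay caches the bar's starting X scale and the player pawn.
; Each tick, IsHuman selects TimeHuman or TimePackage, which sets the bar's X scale as a clamped fraction of 100.
; The bar's shrinkage from its starting scale drives the material's Alpha parameter.
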(event `self.ReceiveBeginPlay`
  (bind _returnvalue_x (`KismetMathLibrary.BreakVector` (`SceneComponent.K2_GetComponentScale` (`self.Bar`))))
  (set `self.InitlaXScale` _returnvalue_x)
  (bind _asthe_player_camera (cast `/Game/Essential/ThePlayerCamera` (`GameplayStatics.GetPlayerPawn` 0)))
  (set `self.ThePlayer` _asthe_player_camera))

(event `self.ReceiveTick`
  (params (DeltaSeconds :type "Float (single-precision)"))
  (bind _theplayer (`self.ThePlayer`))
  (bind _bar (`self.Bar`))
  (bind _returnvalue_x (`KismetMathLibrary.BreakVector` (`SceneComponent.K2_GetComponentScale` _bar)))
  (bind (_returnvalue_x_2 _returnvalue_y _returnvalue_z) (`KismetMathLibrary.BreakVector` (`SceneComponent.K2_GetComponentScale` (`self.Bar`))))
  (if (`self.IsHuman`)
    (set `self.CurrentTime` (`/Game/Essential/ThePlayerCamera.TimeHuman` _theplayer))
    (else
      (set `self.CurrentTime` (`/Game/Essential/ThePlayerCamera.TimePackage` _theplayer))))
  (`SceneComponent.SetWorldScale3D` (`self.Bar`) (`KismetMathLibrary.MakeVector` (`KismetMathLibrary.FClamp` (/ (`self.CurrentTime`) 100.0)) _returnvalue_y _returnvalue_z))
  (`MeshComponent.SetScalarParameterValueOnMaterials` _bar "Alpha" (- 1.0 (/ _returnvalue_x (`self.InitlaXScale`)))))

(fn `UserConstructionScript`)