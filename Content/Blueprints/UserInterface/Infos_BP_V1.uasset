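; Info board actor that shows which human types (traveler, worker, student) and box colors (red, blue, black) are currently forbidden.
; On BeginPlay it caches the ThePlayerCamera pawn and fills its six text components from variables.
; Clicked calls ConstructInfos, which shows each text only if the matching forbidden flag on the pawn is set, then has the pawn play its info animation.
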(event `self.ReceiveBeginPlay`
  (bind _asthe_player_camera (cast `/Game/Essential/ThePlayerCamera` (`GameplayStatics.GetPlayerPawn` 0)))
  (set `self.ThePlayer` _asthe_player_camera)
  ;[1 1 1] InitializeFields
  (`TextRenderComponent.K2_SetText` (`self.Pour les colis1`) (`self.Colis1`))
  (`TextRenderComponent.K2_SetText` (`self.Pour les colis2`) (`self.Colis2`))
  (`TextRenderComponent.K2_SetText` (`self.Pour les colis3`) (`self.Colis3`))
  (`TextRenderComponent.K2_SetText` (`self.Pour les humains1`) (`self.Humain1`))
  (`TextRenderComponent.K2_SetText` (`self.Pour les humains2`) (`self.Humain2`))
  (`TextRenderComponent.K2_SetText` (`self.Pour les humains3`) (`self.Humain3`)))

(event `/Game/Blueprints/ClickedEvent.Clicked`
  (`self.ConstructInfos`)
  (`/Game/Essential/ThePlayerCamera.PlayAnimationInfos` (`self.ThePlayer`)))

(event `ConstructInfos`
  (bind _theplayer (`self.ThePlayer`))
  (`SceneComponent.SetVisibility` (`self.Pour les humains1`) (`/Game/Essential/ThePlayerCamera.TravelerForbidden` _theplayer) false)
  (`SceneComponent.SetVisibility` (`self.Pour les humains2`) (`/Game/Essential/ThePlayerCamera.WorkerForbidden` _theplayer) false)
  (`SceneComponent.SetVisibility` (`self.Pour les humains3`) (`/Game/Essential/ThePlayerCamera.StudentForbidden` _theplayer) false)
  (`SceneComponent.SetVisibility` (`self.Pour les colis1`) (`/Game/Essential/ThePlayerCamera.RedBoxesForbidden` _theplayer) false)
  (`SceneComponent.SetVisibility` (`self.Pour les colis2`) (`/Game/Essential/ThePlayerCamera.BlueBoxForbidden` _theplayer) false)
  (`SceneComponent.SetVisibility` (`self.Pour les colis3`) (`/Game/Essential/ThePlayerCamera.BlackBoxForbidden` _theplayer) false))

(fn `UserConstructionScript`)