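; ClickableButton_BP is a clickable yes/no mesh button that answers either the human or the carpet held by the player camera pawn.
; The construction script gives the static mesh a check or cross material based on IsYes.
; BeginPlay caches the ThePlayerCamera pawn, and Clicked uses IsHuman and IsYes to call Yes or No on its TheHuman or TheCarpet reference.
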(event `self.ReceiveBeginPlay`
  (bind _asthe_player_camera (cast `/Game/Essential/ThePlayerCamera` (`GameplayStatics.GetPlayerPawn` 0)))
  (set `self.ThePlayer` _asthe_player_camera))

(event `/Game/Blueprints/ClickedEvent.Clicked`
  (bind _thecarpet (`/Game/Essential/ThePlayerCamera.TheCarpet` (`self.ThePlayer`)))
  (bind _thehuman (`/Game/Essential/ThePlayerCamera.TheHuman` (`self.ThePlayer`)))
  (if (`self.IsHuman`)
    (if (`self.IsYes`)
      (`/Game/Blueprints/AI/HumanSpawner_BP.Yes` _thehuman)
      (else
        (`/Game/Blueprints/AI/HumanSpawner_BP.No` _thehuman)))
    (elif (`self.IsYes`)
      (`/Game/Blueprints/SlidingCarpet/SlindingCarpet_BP.Yes` _thecarpet)
      (else
        (`/Game/Blueprints/SlidingCarpet/SlindingCarpet_BP.No` _thecarpet)))))

(fn `UserConstructionScript`
  (bind _staticmesh (`self.StaticMesh`))
  (if (`self.IsYes`)
    (`PrimitiveComponent.SetMaterial` _staticmesh 0 "/Game/Assets/MaterialAndTextures/Materiaux/BaseTexture/Childs/BT_Check.BT_Check")
    (else
      (`PrimitiveComponent.SetMaterial` _staticmesh 0 "/Game/Assets/MaterialAndTextures/Materiaux/BaseTexture/Childs/BT_Cross.BT_Cross"))))