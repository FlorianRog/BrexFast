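; PackageDescription_BP is a clickable in-world label that shows a package's type and sender ("De").
; Its construction script builds two text render strings from the PackageType and From variables.
; It caches the ThePlayerCamera pawn on BeginPlay, and a click tells that pawn to play its package description animation.
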(event `self.ReceiveBeginPlay`
  (bind _asthe_player_camera (cast `/Game/Essential/ThePlayerCamera` (`GameplayStatics.GetPlayerPawn` 0)))
  (set `self.ThePlayer` _asthe_player_camera))

(event `/Game/Blueprints/ClickedEvent.Clicked`
  (`/Game/Essential/ThePlayerCamera.PlayAnimationDescriptionPackage` (`self.ThePlayer`)))

(fn `UserConstructionScript`
  (`TextRenderComponent.K2_SetText` (`self.TextRender`) (`KismetTextLibrary.Conv_StringToText` (`KismetStringLibrary.Concat_StrStr` "Type : " (`self.PackageType`))))
  (`TextRenderComponent.K2_SetText` (`self.TextRender1`) (`KismetTextLibrary.Conv_StringToText` (`KismetStringLibrary.Concat_StrStr` "De : " (`self.From`)))))