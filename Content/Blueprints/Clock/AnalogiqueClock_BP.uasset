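; AnalogiqueClock_BP is an in-game clock that, despite its name, displays the time as zero-padded HH:MM text.
; On BeginPlay it caches MyPlayerController and registers itself there as TheClockForTheEnd.
; Every Tick it rounds the controller's LHeure and LesMinutes values, builds the string and writes it to the Hour text.
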(event `self.ReceiveBeginPlay`
  (bind _asmy_player_controller (cast `/Game/Essential/MyPlayerController` (`GameplayStatics.GetPlayerController` 0)))
  (bind _output_get (set `self.ThePlayerController` _asmy_player_controller))
  (set `/Game/Essential/MyPlayerController.TheClockForTheEnd` self _output_get))

(event `self.ReceiveTick`
  (params (DeltaSeconds :type "Float (single-precision)"))
  (bind _theplayercontroller (`self.ThePlayerController`))
  (bind _thehour (`self.TheHour`))
  (bind _returnvalue (`KismetMathLibrary.Round` (`/Game/Essential/MyPlayerController.LesMinutes` _theplayercontroller)))
  (bind _returnvalue_2 (`KismetMathLibrary.Round` (`/Game/Essential/MyPlayerController.L'Heure` _theplayercontroller)))
  (bind _returnvalue_3 (`KismetStringLibrary.Conv_IntToString` _returnvalue))
  (bind _returnvalue_4 (`KismetStringLibrary.Conv_IntToString` _returnvalue_2))
  ;[1 1 1] Change le texte de l'horloge
  (`/Engine/EditorBlueprintResources/StandardMacros.IsValid` _theplayercontroller
    (:`Is Valid`
      (set `self.TheHour` (select `bool` (< _returnvalue_2 10) :`false` _returnvalue_4 :`true` (`KismetStringLibrary.Concat_StrStr` "0" _returnvalue_4)))
      (set `self.TheHour` (`KismetStringLibrary.Concat_StrStr` (`self.TheHour`) " : "))
      (set `self.TheHour` (select `bool` (< _returnvalue 10) :`false` (`KismetStringLibrary.Concat_StrStr` _thehour _returnvalue_3) :`true` (`KismetStringLibrary.Concat_StrStr` _thehour "0" _returnvalue_3)))
      (`TextRenderComponent.K2_SetText` (`self.Hour`) (`KismetTextLibrary.Conv_StringToText` (`self.TheHour`))))))

(fn `UserConstructionScript`)