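; Clock actor whose hour and minute hands display the time held by the player controller.
; On BeginPlay it caches the first player controller as MyPlayerController and clears that controller's TheClockForTheEnd reference.
; Each Tick, while the controller is valid, it converts LHeure and LesMinutes into relative roll rotations for ClockHour and ClockMinute.
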(event `self.ReceiveBeginPlay`
  (bind _asmy_player_controller (cast `/Game/Essential/MyPlayerController` (`GameplayStatics.GetPlayerController` 0)))
  (bind _output_get (set `self.ThePlayerController` _asmy_player_controller))
  (set `/Game/Essential/MyPlayerController.TheClockForTheEnd` null _output_get))

(event `self.ReceiveTick`
  (params (DeltaSeconds :type "Float (single-precision)"))
  (bind _theplayercontroller (`self.ThePlayerController`))
  ;[1 1 1] Change la rotation des aiguilles
  (`/Engine/EditorBlueprintResources/StandardMacros.IsValid` _theplayercontroller
    (:`Is Valid`
      ;;[1 1 1] Change la rotation de l'heure (Angles + 30°)
      (`SceneComponent.K2_SetRelativeRotation` (`self.ClockHour`) (`KismetMathLibrary.MakeRotator` (* (`/Game/Essential/MyPlayerController.L'Heure` _theplayercontroller) -30.0)) false false)
      ;;[1 1 1] Change la rotation des minutes (Angle + 6°)
      (`SceneComponent.K2_SetRelativeRotation` (`self.ClockMinute`) (`KismetMathLibrary.MakeRotator` (* (`/Game/Essential/MyPlayerController.LesMinutes` _theplayercontroller) -6.0)) false false))))

(fn `UserConstructionScript`)