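; Conveyor carpet for a box-sorting game that spawns random colored boxes and moves them on Tick.
; InTraitment overlap halts the belt and spawning, holding the box for a decision.
; Yes sends it along YesDirection and No launches it upward, both updating the player's package gauge from color-is-bad flags and re-enabling spawning.
; Destruction boxes destroy arriving boxes and restore the normal direction; No checks the green flag for black boxes.
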(event `self.ReceiveBeginPlay`
  (bind _asthe_player_camera (cast `/Game/Essential/ThePlayerCamera` (`GameplayStatics.GetPlayerPawn` 0)))
  (bind _output_get (set `self.ThePlayer` _asthe_player_camera))
  (set `/Game/Essential/ThePlayerCamera.TheCarpet` self _output_get)
  (set `self.TheDirection` (`self.NormalDirection`))
  (set `self.BoxForMovements` (`self.NormalMovementBox`))
  (`self.SpawnBoxes`)
  (`KismetSystemLibrary.K2_SetTimerDelegate` (delegate `SpawnBoxes`) 0.2 true))

(event `self.ReceiveTick`
  (params (DeltaSeconds :type "Float (single-precision)"))
  (for _array_element (`PrimitiveComponent.GetOverlappingActors` (`self.BoxForMovements`) "/Game/Blueprints/SlidingCarpet/Boxes/BoxParent.BoxParent_C")
    (if (!= _array_element self)
      (`self.K2_AddActorWorldOffset` _array_element (* (`SceneComponent.GetForwardVector` (`self.TheDirection`)) (* DeltaSeconds (`self.Speed`))) false false))))

(event `self.DestructionBox.OnComponentBeginOverlap`
  (params (OverlappedComponent :type "PrimitiveComponent Object Reference") (OtherActor :type "Actor Object Reference") (OtherComp :type "PrimitiveComponent Object Reference") (OtherBodyIndex :type Integer) (bFromSweep :type Boolean) (SweepResult :type "HitResult Structure (by ref)"))
  (bind _asbox_parent (cast `/Game/Blueprints/SlidingCarpet/Boxes/BoxParent` OtherActor))
  (`self.K2_DestroyActor` _asbox_parent)
  (`self.SetActorTickEnabled` false :!label _label)
  (set `self.TheDirection` (`self.NormalDirection`))
  (set `self.BoxForMovements` (`self.NormalMovementBox`))
  (`self.SetActorTickEnabled` true))

(event `SpawnBoxes`
  (bind _returnvalue (`SceneComponent.K2_GetComponentToWorld` (`self.PlaceToSpawn`)))
  (if (`self.CanSpawn`)
    (`KismetSystemLibrary.Delay` 0.3)
    (switch `int` (`KismetMathLibrary.RandomIntegerInRange` 0 4)
      (:`0`
        (bind _returnvalue_2 (`|SpawnActorFromClass` "/Game/Blueprints/SlidingCarpet/Boxes/GreenBox_BP.GreenBox_BP_C" _returnvalue "Undefined" "OverrideRootScale" null null))
        (set `self.SpawnedBox` _returnvalue_2))
      (:`1`
        (bind _returnvalue_3 (`|SpawnActorFromClass` "/Game/Blueprints/SlidingCarpet/Boxes/RedBox_BP.RedBox_BP_C" _returnvalue "Undefined" "OverrideRootScale" null null))
        (set `self.SpawnedBox` _returnvalue_3))
      (:`2`
        (bind _returnvalue_4 (`|SpawnActorFromClass` "/Game/Blueprints/SlidingCarpet/Boxes/BlueBox_BP.BlueBox_BP_C" _returnvalue "Undefined" "OverrideRootScale" null null))
        (set `self.SpawnedBox` _returnvalue_4))
      (:`3`
        (bind _returnvalue_5 (`|SpawnActorFromClass` "/Game/Blueprints/SlidingCarpet/Boxes/WhiteBox_BP.WhiteBox_BP_C" _returnvalue "Undefined" "OverrideRootScale" null null))
        (set `self.SpawnedBox` _returnvalue_5))
      (:`4`
        (bind _returnvalue_6 (`|SpawnActorFromClass` "/Game/Blueprints/SlidingCarpet/Boxes/BlackBox_BP.BlackBox_BP_C" _returnvalue "Undefined" "OverrideRootScale" null null))
        (set `self.SpawnedBox` _returnvalue_6)))))

(event `self.DestructionBox1.OnComponentBeginOverlap`
  (params (OverlappedComponent :type "PrimitiveComponent Object Reference") (OtherActor :type "Actor Object Reference") (OtherComp :type "PrimitiveComponent Object Reference") (OtherBodyIndex :type Integer) (bFromSweep :type Boolean) (SweepResult :type "HitResult Structure (by ref)"))
  (bind _asbox_parent (cast `/Game/Blueprints/SlidingCarpet/Boxes/BoxParent` OtherActor))
  (`self.K2_DestroyActor` _asbox_parent)
  (goto _label))

(event `self.InTraitment.OnComponentBeginOverlap`
  (params (OverlappedComponent :type "PrimitiveComponent Object Reference") (OtherActor :type "Actor Object Reference") (OtherComp :type "PrimitiveComponent Object Reference") (OtherBodyIndex :type Integer) (bFromSweep :type Boolean) (SweepResult :type "HitResult Structure (by ref)"))
  (if (!= OtherActor (`self.TheBox`))
    (bind _asbox_parent (cast `/Game/Blueprints/SlidingCarpet/Boxes/BoxParent` OtherActor))
    (set `self.CanSpawn` false)
    (bind _output_get (set `self.TheBox` _asbox_parent))
    (`self.SetActorTickEnabled` false)
    (`KismetSystemLibrary.MoveComponentTo` (`/Game/Blueprints/SlidingCarpet/Boxes/BoxParent.TheBox` _output_get) (`SceneComponent.K2_GetComponentLocation` (`self.InTraitment`)))
    (`/Engine/EditorBlueprintResources/StandardMacros.DoOnce` false
      (:`Completed`
        (`/Game/Essential/ThePlayerCamera.BaisseJaugePackage` (`self.ThePlayer`))))))

(fn `No`
  (bind _thebox (`self.TheBox`))
  (bind _theplayer (`self.ThePlayer`))
  (`/Engine/EditorBlueprintResources/StandardMacros.IsValid` _thebox
    (:`Is Valid`
      (cast `/Game/Blueprints/SlidingCarpet/Boxes/GreenBox_BP` _thebox
        (:`then`
          (if (`/Game/Essential/ThePlayerCamera.GreenBoxesAreBad` (`self.ThePlayer`))
            (`/Game/Essential/ThePlayerCamera.ChangeJaugePackage` _theplayer false :!label _label)
            (else
              (`/Game/Essential/ThePlayerCamera.ChangeJaugePackage` _theplayer true :!label _label_2))))
        (:`CastFailed`
          (cast `/Game/Blueprints/SlidingCarpet/Boxes/RedBox_BP` _thebox
            (:`then`
              (if (`/Game/Essential/ThePlayerCamera.RedBoxesAreBad` (`self.ThePlayer`))
                (goto _label)
                (else
                  (goto _label_2))))
            (:`CastFailed`
              (cast `/Game/Blueprints/SlidingCarpet/Boxes/BlueBox_BP` _thebox
                (:`then`
                  (if (`/Game/Essential/ThePlayerCamera.BlueBoxesAreBad` (`self.ThePlayer`))
                    (goto _label)
                    (else
                      (goto _label_2))))
                (:`CastFailed`
                  (cast `/Game/Blueprints/SlidingCarpet/Boxes/WhiteBox_BP` _thebox
                    (:`then`
                      (if (`/Game/Essential/ThePlayerCamera.WhiteBoxesAreBad` (`self.ThePlayer`))
                        (goto _label)
                        (else
                          (goto _label_2))))
                    (:`CastFailed`
                      (cast `/Game/Blueprints/SlidingCarpet/Boxes/BlackBox_BP` _thebox)
                      (if (`/Game/Essential/ThePlayerCamera.GreenBoxesAreBad` (`self.ThePlayer`))
                        (goto _label)
                        (else
                          (goto _label_2)))))))))))
      (`PrimitiveComponent.AddImpulse` (`/Game/Blueprints/SlidingCarpet/Boxes/BoxParent.TheBox` (`self.TheBox`)) (0.0 0.0 5000000.0) "None" false)
      (set `self.CanSpawn` true))))

(fn `UserConstructionScript`)

(fn `Yes`
  (bind _thebox (`self.TheBox`))
  (bind _theplayer (`self.ThePlayer`))
  (`/Engine/EditorBlueprintResources/StandardMacros.IsValid` _thebox
    (:`Is Valid`
      (cast `/Game/Blueprints/SlidingCarpet/Boxes/GreenBox_BP` _thebox
        (:`then`
          (if (`/Game/Essential/ThePlayerCamera.GreenBoxesAreBad` (`self.ThePlayer`))
            (`/Game/Essential/ThePlayerCamera.ChangeJaugePackage` _theplayer true :!label _label)
            (else
              (`/Game/Essential/ThePlayerCamera.ChangeJaugePackage` _theplayer false :!label _label_2))))
        (:`CastFailed`
          (cast `/Game/Blueprints/SlidingCarpet/Boxes/RedBox_BP` _thebox
            (:`then`
              (if (`/Game/Essential/ThePlayerCamera.RedBoxesAreBad` (`self.ThePlayer`))
                (goto _label)
                (else
                  (goto _label_2))))
            (:`CastFailed`
              (cast `/Game/Blueprints/SlidingCarpet/Boxes/BlueBox_BP` _thebox
                (:`then`
                  (if (`/Game/Essential/ThePlayerCamera.BlueBoxesAreBad` (`self.ThePlayer`))
                    (goto _label)
                    (else
                      (goto _label_2))))
                (:`CastFailed`
                  (cast `/Game/Blueprints/SlidingCarpet/Boxes/WhiteBox_BP` _thebox
                    (:`then`
                      (if (`/Game/Essential/ThePlayerCamera.WhiteBoxesAreBad` (`self.ThePlayer`))
                        (goto _label)
                        (else
                          (goto _label_2))))
                    (:`CastFailed`
                      (cast `/Game/Blueprints/SlidingCarpet/Boxes/BlackBox_BP` _thebox)
                      (if (`/Game/Essential/ThePlayerCamera.BlackBoxesAreBad` (`self.ThePlayer`))
                        (goto _label)
                        (else
                          (goto _label_2)))))))))))
      (set `self.TheDirection` (`self.YesDirection`))
      (set `self.BoxForMovements` (`self.InTraitment`))
      (`self.SetActorTickEnabled` true)
      (set `self.CanSpawn` true))))