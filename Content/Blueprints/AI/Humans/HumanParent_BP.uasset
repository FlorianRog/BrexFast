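; Base AI human for a document-checking game, randomized in appearance, name, travel type and stay duration.
; Construction randomizes gender, mesh and materials; BeginPlay draws identity from data tables.
; The player's current day selects a check that chains through earlier days' rules, rolling papers by percentage and ANDing results into IsAGoodHuman.
; A front box clears blackboard CanMove while overlapping another human; GiveHumanParams exposes the document flags.
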(event `self.BoxFront.OnComponentEndOverlap`
  (params (OverlappedComponent :type "PrimitiveComponent Object Reference") (OtherActor :type "Actor Object Reference") (OtherComp :type "PrimitiveComponent Object Reference") (OtherBodyIndex :type Integer))
  (cast `/Game/Blueprints/AI/Humans/HumanParent_BP` OtherActor)
  (`/Engine/EditorBlueprintResources/StandardMacros.IsValid` self
    (:`Is Valid`
      (`BlackboardComponent.SetValueAsBool` (`AIBlueprintHelperLibrary.GetBlackboard` self) "CanMove" true))))

(event `self.BoxFront.OnComponentBeginOverlap`
  (params (OverlappedComponent :type "PrimitiveComponent Object Reference") (OtherActor :type "Actor Object Reference") (OtherComp :type "PrimitiveComponent Object Reference") (OtherBodyIndex :type Integer) (bFromSweep :type Boolean) (SweepResult :type "HitResult Structure (by ref)"))
  (cast `/Game/Blueprints/AI/Humans/HumanParent_BP` OtherActor)
  (`/Engine/EditorBlueprintResources/StandardMacros.IsValid` self
    (:`Is Valid`
      (`BlackboardComponent.SetValueAsBool` (`AIBlueprintHelperLibrary.GetBlackboard` self) "CanMove" false))))

(event `self.ReceiveBeginPlay`
  (bind _asthe_player_camera (cast `/Game/Essential/ThePlayerCamera` (`GameplayStatics.GetPlayerPawn` 0)))
  (set `self.ThePlayer` _asthe_player_camera)
  ;[1 1 1] Set the travel type
  (bind _outrownames (`DataTableFunctionLibrary.GetDataTableRowNames` "/Game/Blueprints/Databases/Humans/DB_TravelType.DB_TravelType"))
  (set `self.RandomTravelTypeID` (`KismetMathLibrary.RandomIntegerInRange` 0 (- (`KismetArrayLibrary.Array_Length` _outrownames) 1)))
  (for (_array_element _array_index) _outrownames
    (if (== _array_index (`self.RandomTravelTypeID`))
      (bind _returnvalue (`|GetDataTableRow` "/Game/Blueprints/Databases/Humans/DB_TravelType.DB_TravelType" _array_element)
        (:`then`
          (bind (_traveltype _isaworker _isastudent _isatraveler _isamigrant) (break `/Game/Blueprints/Databases/Humans/STDT_TravelType` _returnvalue))
          (set `self.TravelType` _traveltype)
          (set `self.IsAWorker` _isaworker)
          (set `self.IsAStudent` _isastudent)
          (set `self.IsATraveler` _isatraveler)
          (set `self.IsAMigrant` _isamigrant)))))
  (if (`self.IsAMigrant`)
    (set `self.Duration` "Toujours")
    (set `self.IsALongJourney` true)
    (else
      ;[1 1 1] Get a duration
      (bind _outrownames_2 (`DataTableFunctionLibrary.GetDataTableRowNames` "/Game/Blueprints/Databases/Humans/BD_Duration.BD_Duration"))
      (set `self.RandomDurationID` (`KismetMathLibrary.RandomIntegerInRange` 0 (- (`KismetArrayLibrary.Array_Length` _outrownames_2) 1)))
      (for (_array_element_2 _array_index_2) _outrownames_2
        (if (== _array_index_2 (`self.RandomDurationID`))
          (bind _returnvalue_2 (`|GetDataTableRow` "/Game/Blueprints/Databases/Humans/BD_Duration.BD_Duration" _array_element_2)
            (:`then`
              (bind (_duration _islong) (break `/Game/Blueprints/Databases/Humans/STDT_Duration` _returnvalue_2))
              (set `self.Duration` _duration)
              (set `self.IsALongJourney` _islong)))))))
  ;[1 1 1] Pick a random name
  (if (`self.IsMale`)
    (bind _outrownames_3 (`DataTableFunctionLibrary.GetDataTableRowNames` "/Game/Blueprints/Databases/Humans/BD_PrenomMale.BD_PrenomMale"))
    (set `self.RandomNameID` (- (`KismetMathLibrary.RandomIntegerInRange` 0 (`KismetArrayLibrary.Array_Length` _outrownames_3)) 1))
    (for (_array_element_3 _array_index_3) _outrownames_3
      (if (== _array_index_3 (`self.RandomNameID`))
        (bind _returnvalue_3 (`|GetDataTableRow` "/Game/Blueprints/Databases/Humans/BD_PrenomMale.BD_PrenomMale" _array_element_3)
          (:`then`
            (set `self.Prenom` (`.Prenom_5_923AD7C849F9D4EE403BC28E32FA6A51` (break `/Game/Blueprints/Databases/Humans/STDT_PrenomMale` _returnvalue_3)))
            (switch `int` (`/Game/Essential/ThePlayerCamera.CurrentDay` (`self.ThePlayer`)) :!label _label
              (:`Default`
                (`self.CheckDiplomeMigrant` :!label _label_2))
              (:`1`
                (`self.CheckIDPapers`))
              (:`2`
                (`self.CheckCitizenshipPapers`))
              (:`3`
                (`self.CheckVisaWorker`))
              (:`4`
                (`self.CheckVisaStudent`))
              (:`5`
                (`self.CheckVisaTraveler`))
              (:`6`
                (`self.ChangePercentIDAndPP`))
              (:`7`
                (`self.CheckImmigrantAptitude`))
              (:`8`
                (`self.CheckPermisDeSejour`))
              (:`9`
                (`self.CheckHaveAssurance`))
              (:`10`
                (`self.CheckWorkPermis`))
              (:`11`
                (goto _label_2)))))))
    (else
      (bind _outrownames_4 (`DataTableFunctionLibrary.GetDataTableRowNames` "/Game/Blueprints/Databases/Humans/BD_PrenomFemale.BD_PrenomFemale"))
      (set `self.RandomNameID` (- (`KismetMathLibrary.RandomIntegerInRange` 0 (`KismetArrayLibrary.Array_Length` _outrownames_4)) 1))
      (for (_array_element_4 _array_index_4) _outrownames_4
        (if (== _array_index_4 (`self.RandomNameID`))
          (bind _returnvalue_4 (`|GetDataTableRow` "/Game/Blueprints/Databases/Humans/BD_PrenomFemale.BD_PrenomFemale" _array_element_4)
            (:`then`
              (set `self.Prenom` (`.Prenom_5_923AD7C849F9D4EE403BC28E32FA6A51` (break `/Game/Blueprints/Databases/Humans/STDT_PrenomFemale` _returnvalue_4)))
              (goto _label))))))))

(event `SetGoodHuman`
  ;[1 1 1] Directive change stat
  ;;[1 1 1] Set is a good human
  (for _array_element (`self.IsInGoodWay`)
    (set `self.IsAGoodHuman` (and _array_element (`self.IsAGoodHuman`)))))

(event `CheckIDPapers`
  (bind _isingoodway (`self.IsInGoodWay`))
  (bind _returnvalue (<= (`self.RandomFloatForChecks`) (+ (`self.PercentToHaveID`) (`self.PercentToHavePasseport`))))
  ;[1 1 1] Directive change stat
  ;;[1 1 1] CheckIDPapers
  (bind _output_get (set `self.RandomFloatForChecks` (`KismetMathLibrary.RandomFloatInRange` 0.0 100.0)))
  (if (<= _output_get (`self.PercentToHaveID`))
    (set `self.HaveID` true)
    (`KismetArrayLibrary.Array_Add` _isingoodway (not (`self.IDForbidden`)))
    (else
      (set `self.HavePP` _returnvalue)
      (`KismetArrayLibrary.Array_Add` _isingoodway _returnvalue)))
  (`self.SetGoodHuman`))

(event `CheckCitizenshipPapers`
  ;[1 1 1] Directive change stat
  ;;[1 1 1] CheckCitizensPapers
  (if (`self.IsAMigrant`)
    (bind _output_get (set `self.RandomFloatForChecks` (`KismetMathLibrary.RandomFloatInRange` 0.0 100.0)))
    (bind _output_get_2 (set `self.HaveCS` (<= _output_get (`self.PercentToHaveCitizenshipPaper`))))
    (`KismetArrayLibrary.Array_Add` (`self.IsInGoodWay`) _output_get_2)
    (`self.CheckIDPapers`)
    (else
      (`self.CheckIDPapers`))))

(event `CheckVisaWorker`
  ;[1 1 1] Directive change stat
  ;;[1 1 1] Check visa worker
  (if (and (`self.IsAWorker`) (`self.IsALongJourney`))
    (bind _output_get (set `self.RandomFloatForChecks` (`KismetMathLibrary.RandomFloatInRange` 0.0 100.0)))
    (bind _output_get_2 (set `self.HaveVisaW` (<= _output_get (`self.PercentWorkerHaveVisa`))))
    (`KismetArrayLibrary.Array_Add` (`self.IsInGoodWay`) _output_get_2)
    (`self.CheckCitizenshipPapers`)
    (else
      (`self.CheckCitizenshipPapers`))))

(event `CheckVisaStudent`
  ;[1 1 1] Directive change stat
  ;;[1 1 1] CheckVisaStudent
  (if (and (`self.IsAStudent`) (`self.IsALongJourney`))
    (bind _output_get (set `self.RandomFloatForChecks` (`KismetMathLibrary.RandomFloatInRange` 0.0 100.0)))
    (bind _output_get_2 (set `self.HaveVisaS` (<= _output_get (`self.PercentStudentHaveVisa`))))
    (`KismetArrayLibrary.Array_Add` (`self.IsInGoodWay`) _output_get_2)
    (`self.CheckVisaWorker`)
    (else
      (`self.CheckVisaWorker`))))

(event `CheckVisaTraveler`
  ;[1 1 1] Directive change stat
  ;;[1 1 1] CheckVisaTraveler
  (if (and (`self.IsATraveler`) (`self.IsALongJourney`))
    (bind _output_get (set `self.RandomFloatForChecks` (`KismetMathLibrary.RandomFloatInRange` 0.0 100.0)))
    (bind _output_get_2 (set `self.HaveVisaT` (<= _output_get (`self.PercentTravelerHaveVisa`))))
    (`KismetArrayLibrary.Array_Add` (`self.IsInGoodWay`) _output_get_2)
    (`self.CheckVisaStudent`)
    (else
      (`self.CheckVisaStudent`))))

(event `ChangePercentIDAndPP`
  ;[1 1 1] Directive change stat
  ;;[1 1 1] ChangePercentIDandPP
  (set `self.PercentToHaveID` 20.0)
  (set `self.PercentToHavePasseport` 70.0)
  (set `self.IDForbidden` true)
  (`self.CheckVisaTraveler`))

(event `CheckImmigrantAptitude`
  ;[1 1 1] Directive change stat
  ;;[1 1 1] CheckImmigrantAptitude
  (if (`self.IsAMigrant`)
    (bind _output_get (set `self.RandomFloatForChecks` (`KismetMathLibrary.RandomFloatInRange` 0.0 100.0)))
    (bind _output_get_2 (set `self.HaveAptitude` (<= _output_get (`self.PercentToHaveAptitude`))))
    (`KismetArrayLibrary.Array_Add` (`self.IsInGoodWay`) _output_get_2)
    (`self.ChangePercentIDAndPP`)
    (else
      (`self.ChangePercentIDAndPP`))))

(event `CheckPermisDeSejour`
  ;[1 1 1] Directive change stat
  ;;[1 1 1] Check permis WorkerAndtraveler
  (if (and (or (`self.IsAWorker`) (`self.IsATraveler`)) (`self.IsALongJourney`))
    (bind _output_get (set `self.RandomFloatForChecks` (`KismetMathLibrary.RandomFloatInRange` 0.0 100.0)))
    (bind _output_get_2 (set `self.HavePermis` (<= _output_get (`self.PercentToHavePermis`))))
    (`KismetArrayLibrary.Array_Add` (`self.IsInGoodWay`) _output_get_2)
    (`self.CheckImmigrantAptitude`)
    (else
      (`self.CheckImmigrantAptitude`))))

(event `CheckHaveAssurance`
  ;[1 1 1] Directive change stat
  ;;[1 1 1] CheckAssurance
  (bind _output_get (set `self.RandomFloatForChecks` (`KismetMathLibrary.RandomFloatInRange` 0.0 100.0)))
  (bind _output_get_2 (set `self.HaveAssurance` (<= _output_get (`self.PercentToHaveAssurance`))))
  (`KismetArrayLibrary.Array_Add` (`self.IsInGoodWay`) _output_get_2)
  (`self.CheckPermisDeSejour`))

(event `CheckWorkPermis`
  ;[1 1 1] Directive change stat
  ;;[1 1 1] CheckWorkPermis
  (if (`self.IsAWorker`)
    (bind _output_get (set `self.RandomFloatForChecks` (`KismetMathLibrary.RandomFloatInRange` 0.0 100.0)))
    (bind _output_get_2 (set `self.HavePermisTravail` (<= _output_get (`self.PercentToHaveWorkPermis`))))
    (`KismetArrayLibrary.Array_Add` (`self.IsInGoodWay`) _output_get_2)
    (`self.CheckHaveAssurance`)
    (else
      (`self.CheckHaveAssurance`))))

(event `CheckDiplomeMigrant`
  ;[1 1 1] Directive change stat
  ;;[1 1 1] CheckDiplomeMigrant
  (if (`self.IsAMigrant`)
    (bind _output_get (set `self.RandomFloatForChecks` (`KismetMathLibrary.RandomFloatInRange` 0.0 100.0)))
    (bind _output_get_2 (set `self.HaveDiplome` (<= _output_get (`self.PercentToHaveDiplome`))))
    (`KismetArrayLibrary.Array_Add` (`self.IsInGoodWay`) _output_get_2)
    (`self.CheckWorkPermis`)
    (else
      (`self.CheckWorkPermis`))))

(fn `GiveHumanParams`
  (returns (HaveID :type Boolean) (HavePP :type Boolean) (HaveCS :type Boolean) (HaveVisaW :type Boolean) (HaveVisaS :type Boolean) (HaveVisaT :type Boolean) (HaveAptitude :type Boolean) (HavePermis :type Boolean) (HaveAssurance :type Boolean) (HavePermisTravail :type Boolean) (HaveDiplome :type Boolean))
  (return (`self.HaveID`) (`self.HavePP`) (`self.HaveCS`) (`self.HaveVisaW`) (`self.HaveVisaS`) (`self.HaveVisaT`) (`self.HaveAptitude`) (`self.HavePermis`) (`self.HaveAssurance`) (`self.HavePermisTravail`) (`self.HaveDiplome`)))

(fn `UserConstructionScript`
  (bind _mesh (`self.Mesh`))
  (bind _mesh_2 (`self.Mesh`))
  (bind _mesh_3 (`self.Mesh`))
  (bind _mesh_4 (`self.Mesh`))
  (bind _mesh_5 (`self.Mesh`))
  (bind _mesh_6 (`self.Mesh`))
  (bind _mesh_7 (`self.Mesh`))
  (if (`KismetMathLibrary.RandomBool`)
    (`SkinnedMeshComponent.SetSkinnedAssetAndUpdate` _mesh_4 "/Game/Assets/Humans/Male/Male.Male" true)
    (set `self.IsMale` true)
    ;[1 1 1] Change la couleur de la peau
    (`PrimitiveComponent.SetMaterial` (`self.Mesh`) 0 "/Game/Assets/MaterialAndTextures/Materiaux/BaseTexture/BT_Parent.BT_Parent")
    ;[1 1 1] Change la couleur du tshirt
    (switch `int` (`KismetMathLibrary.RandomIntegerInRange` 0 4)
      (:`Default`
        (`PrimitiveComponent.SetMaterial` _mesh_3 1 "/Game/Assets/MaterialAndTextures/Materiaux/BaseColor/Childs/inst_f7f1e3.inst_f7f1e3" :!label _label))
      (:`0`
        (`PrimitiveComponent.SetMaterial` _mesh_3 1 "/Game/Assets/MaterialAndTextures/Materiaux/BaseColor/Childs/inst_84817a.inst_84817a"))
      (:`1`
        (`PrimitiveComponent.SetMaterial` _mesh_3 1 "/Game/Assets/MaterialAndTextures/Materiaux/BaseColor/Childs/inst_34ace0.inst_34ace0"))
      (:`2`
        (`PrimitiveComponent.SetMaterial` _mesh_3 1 "/Game/Assets/MaterialAndTextures/Materiaux/BaseColor/Childs/inst_ccae62.inst_ccae62"))
      (:`3`
        (`PrimitiveComponent.SetMaterial` _mesh_3 1 "/Game/Assets/MaterialAndTextures/Materiaux/BaseColor/Childs/inst_ff5252.inst_ff5252"))
      (:`4`
        (goto _label)))
    ;[1 1 1] Change la couleur du pantalon
    (switch `int` (`KismetMathLibrary.RandomIntegerInRange` 0 3)
      (:`Default`
        (`PrimitiveComponent.SetMaterial` _mesh 2 "/Game/Assets/MaterialAndTextures/Materiaux/BaseColor/Childs/inst_d1ccc0.inst_d1ccc0" :!label _label_2))
      (:`0`
        (`PrimitiveComponent.SetMaterial` _mesh 2 "/Game/Assets/MaterialAndTextures/Materiaux/BaseColor/Childs/inst_84817a.inst_84817a"))
      (:`1`
        (`PrimitiveComponent.SetMaterial` _mesh 2 "/Game/Assets/MaterialAndTextures/Materiaux/BaseColor/Childs/inst_34ace0.inst_34ace0"))
      (:`2`
        (`PrimitiveComponent.SetMaterial` _mesh 2 "/Game/Assets/MaterialAndTextures/Materiaux/BaseColor/Childs/inst_f7f1e3.inst_f7f1e3"))
      (:`3`
        (goto _label_2)))
    (else
      (`SkinnedMeshComponent.SetSkinnedAssetAndUpdate` _mesh_4 "/Game/Assets/Humans/Female/Female.Female" true)
      (set `self.IsMale` false)
      ;[1 1 1] Change la couleur de la peau
      (`PrimitiveComponent.SetMaterial` (`self.Mesh`) 0 "/Game/Assets/MaterialAndTextures/Materiaux/BaseTexture/BT_Parent.BT_Parent")
      ;[1 1 1] Change la couleur du tshirt
      (switch `int` (`KismetMathLibrary.RandomIntegerInRange` 0 9)
        (:`Default`
          (`PrimitiveComponent.SetMaterial` _mesh_5 1 "/Game/Assets/MaterialAndTextures/Materiaux/BaseColor/Childs/inst_ffb142.inst_ffb142" :!label _label_3))
        (:`0`
          (`PrimitiveComponent.SetMaterial` _mesh_5 1 "/Game/Assets/MaterialAndTextures/Materiaux/BaseColor/Childs/inst_84817a.inst_84817a"))
        (:`1`
          (`PrimitiveComponent.SetMaterial` _mesh_5 1 "/Game/Assets/MaterialAndTextures/Materiaux/BaseColor/Childs/inst_34ace0.inst_34ace0"))
        (:`2`
          (`PrimitiveComponent.SetMaterial` _mesh_5 1 "/Game/Assets/MaterialAndTextures/Materiaux/BaseColor/Childs/inst_ccae62.inst_ccae62"))
        (:`3`
          (`PrimitiveComponent.SetMaterial` _mesh_5 1 "/Game/Assets/MaterialAndTextures/Materiaux/BaseColor/Childs/inst_218c74.inst_218c74"))
        (:`4`
          (`PrimitiveComponent.SetMaterial` _mesh_5 1 "/Game/Assets/MaterialAndTextures/Materiaux/BaseColor/Childs/inst_ff793f.inst_ff793f"))
        (:`5`
          (`PrimitiveComponent.SetMaterial` _mesh_5 1 "/Game/Assets/MaterialAndTextures/Materiaux/BaseColor/Childs/inst_706fd3.inst_706fd3"))
        (:`6`
          (`PrimitiveComponent.SetMaterial` _mesh_5 1 "/Game/Assets/MaterialAndTextures/Materiaux/BaseColor/Childs/inst_474787.inst_474787"))
        (:`7`
          (`PrimitiveComponent.SetMaterial` _mesh_5 1 "/Game/Assets/MaterialAndTextures/Materiaux/BaseColor/Childs/inst_b33939.inst_b33939"))
        (:`8`
          (`PrimitiveComponent.SetMaterial` _mesh_5 1 "/Game/Assets/MaterialAndTextures/Materiaux/BaseColor/Childs/inst_f7f1e3.inst_f7f1e3"))
        (:`9`
          (goto _label_3)))
      ;[1 1 1] Change la couleur du pantalon
      (switch `int` (`KismetMathLibrary.RandomIntegerInRange` 0 3)
        (:`Default`
          (`PrimitiveComponent.SetMaterial` _mesh_6 2 "/Game/Assets/MaterialAndTextures/Materiaux/BaseColor/Childs/inst_ffb142.inst_ffb142" :!label _label_4))
        (:`0`
          (`PrimitiveComponent.SetMaterial` _mesh_6 2 "/Game/Assets/MaterialAndTextures/Materiaux/BaseColor/Childs/inst_34ace0.inst_34ace0"))
        (:`1`
          (`PrimitiveComponent.SetMaterial` _mesh_6 2 "/Game/Assets/MaterialAndTextures/Materiaux/BaseColor/Childs/inst_b33939.inst_b33939"))
        (:`2`
          (`PrimitiveComponent.SetMaterial` _mesh_6 2 "/Game/Assets/MaterialAndTextures/Materiaux/BaseColor/Childs/inst_f7f1e3.inst_f7f1e3"))
        (:`3`
          (goto _label_4)))))
  ;[1 1 1] Change la couleur des chaussures
  (switch `int` (`KismetMathLibrary.RandomIntegerInRange` 0 2)
    (:`Default`
      (`PrimitiveComponent.SetMaterial` _mesh_7 3 "/Game/Assets/MaterialAndTextures/Materiaux/BaseColor/Childs/inst_f7f1e3.inst_f7f1e3" :!label _label_5))
    (:`0`
      (`PrimitiveComponent.SetMaterial` _mesh_7 3 "/Game/Assets/MaterialAndTextures/Materiaux/BaseColor/Childs/inst_84817a.inst_84817a"))
    (:`1`
      (`PrimitiveComponent.SetMaterial` _mesh_7 3 "/Game/Assets/MaterialAndTextures/Materiaux/BaseColor/Childs/inst_ccae62.inst_ccae62"))
    (:`2`
      (goto _label_5)))
  ;[1 1 1] Change la couleur des cheveux
  (switch `int` (`KismetMathLibrary.RandomIntegerInRange` 0 5)
    (:`Default`
      (`PrimitiveComponent.SetMaterial` _mesh_2 4 "/Game/Assets/MaterialAndTextures/Materiaux/BaseColor/Childs/inst_ff793f.inst_ff793f" :!label _label_6))
    (:`0`
      (`PrimitiveComponent.SetMaterial` _mesh_2 4 "/Game/Assets/MaterialAndTextures/Materiaux/BaseColor/Childs/inst_2c2c54.inst_2c2c54"))
    (:`1`
      (`PrimitiveComponent.SetMaterial` _mesh_2 4 "/Game/Assets/MaterialAndTextures/Materiaux/BaseColor/Childs/inst_ffb142.inst_ffb142"))
    (:`2`
      (`PrimitiveComponent.SetMaterial` _mesh_2 4 "/Game/Assets/MaterialAndTextures/Materiaux/BaseColor/Childs/inst_227093.inst_227093"))
    (:`3`
      (`PrimitiveComponent.SetMaterial` _mesh_2 4 "/Game/Assets/MaterialAndTextures/Materiaux/BaseColor/Childs/inst_cd6133.inst_cd6133"))
    (:`4`
      (`PrimitiveComponent.SetMaterial` _mesh_2 4 "/Game/Assets/MaterialAndTextures/Materiaux/BaseColor/Childs/inst_b33939.inst_b33939"))
    (:`5`
      (goto _label_6)))
  (switch `int` (`KismetMathLibrary.RandomIntegerInRange` 0 16)
    (:`0`
      (set `self.MaterialForSkin` "/Game/Assets/MaterialAndTextures/Materiaux/BaseTexture/Childs/Skins/BT_Skin1.BT_Skin1"))
    (:`1`
      (set `self.MaterialForSkin` "/Game/Assets/MaterialAndTextures/Materiaux/BaseTexture/Childs/Skins/BT_Skin2.BT_Skin2"))
    (:`2`
      (set `self.MaterialForSkin` "/Game/Assets/MaterialAndTextures/Materiaux/BaseTexture/Childs/Skins/BT_Skin3.BT_Skin3"))
    (:`3`
      (set `self.MaterialForSkin` "/Game/Assets/MaterialAndTextures/Materiaux/BaseTexture/Childs/Skins/BT_Skin4.BT_Skin4"))
    (:`4`
      (set `self.MaterialForSkin` "/Game/Assets/MaterialAndTextures/Materiaux/BaseTexture/Childs/Skins/BT_Skin5.BT_Skin5"))
    (:`5`
      (set `self.MaterialForSkin` "/Game/Assets/MaterialAndTextures/Materiaux/BaseTexture/Childs/Skins/BT_Skin6.BT_Skin6"))
    (:`6`
      (set `self.MaterialForSkin` "/Game/Assets/MaterialAndTextures/Materiaux/BaseTexture/Childs/Skins/BT_Skin7.BT_Skin7"))
    (:`7`
      (set `self.MaterialForSkin` "/Game/Assets/MaterialAndTextures/Materiaux/BaseTexture/Childs/Skins/BT_Skin8.BT_Skin8"))
    (:`8`
      (set `self.MaterialForSkin` "/Game/Assets/MaterialAndTextures/Materiaux/BaseTexture/Childs/Skins/BT_Skin9.BT_Skin9"))
    (:`9`
      (set `self.MaterialForSkin` "/Game/Assets/MaterialAndTextures/Materiaux/BaseTexture/Childs/Skins/BT_Skin10.BT_Skin10"))
    (:`10`
      (set `self.MaterialForSkin` "/Game/Assets/MaterialAndTextures/Materiaux/BaseTexture/Childs/Skins/BT_Skin11.BT_Skin11"))
    (:`11`
      (set `self.MaterialForSkin` "/Game/Assets/MaterialAndTextures/Materiaux/BaseTexture/Childs/Skins/BT_Skin12.BT_Skin12"))
    (:`12`
      (set `self.MaterialForSkin` "/Game/Assets/MaterialAndTextures/Materiaux/BaseTexture/Childs/Skins/BT_Skin13.BT_Skin13"))
    (:`13`
      (set `self.MaterialForSkin` "/Game/Assets/MaterialAndTextures/Materiaux/BaseTexture/Childs/Skins/BT_Skin14.BT_Skin14"))
    (:`14`
      (set `self.MaterialForSkin` "/Game/Assets/MaterialAndTextures/Materiaux/BaseTexture/Childs/Skins/BT_Skin15.BT_Skin15"))
    (:`15`
      (set `self.MaterialForSkin` "/Game/Assets/MaterialAndTextures/Materiaux/BaseTexture/Childs/Skins/BT_Skin16.BT_Skin16"))
    (:`16`
      (set `self.MaterialForSkin` "/Game/Assets/MaterialAndTextures/Materiaux/BaseTexture/Childs/Skins/BT_Skin17.BT_Skin17")))
  (`PrimitiveComponent.SetMaterial` (`self.Mesh`) 0 (`self.MaterialForSkin`)))