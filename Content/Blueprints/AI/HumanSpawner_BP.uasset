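; Spawns the travelers of a passport-check desk and applies the player's Yes/No verdict on each.
; A random-delay loop spawns NPC_BT-driven humans while the start box is clear, stopping if it is blocked, and sends them via blackboard to the desk.
; Desk overlap has the player pawn show papers and info.
; Verdicts update gauges from IsGoodGuy, then walk the human to a destroy box or spring-launch them upward.
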(event `self.ReceiveBeginPlay`
  ;[1 1 1] Begin play
  (bind _asthe_player_camera (cast `/Game/Essential/ThePlayerCamera` (`GameplayStatics.GetPlayerPawn` 0)))
  (set `self.ThePlayer` _asthe_player_camera)
  (set `/Game/Essential/ThePlayerCamera.TheHuman` self _asthe_player_camera)
  (bind _asspring_bp (cast `/Game/Blueprints/Spring/Spring_Bp` (`ChildActorComponent.ChildActor` (`self.Spring`))))
  (set `self.MySpring` _asspring_bp)
  (`self.SpawnPeople`))

(event `self.BoxStart.OnComponentEndOverlap`
  (params (OverlappedComponent :type "PrimitiveComponent Object Reference") (OtherActor :type "Actor Object Reference") (OtherComp :type "PrimitiveComponent Object Reference") (OtherBodyIndex :type Integer))
  ;[1 1 1] Verifie que rien n'est en collision aveec la boite de spawn
  (set `self.CanSpawn` true))

(event `SpawnPeople`
  ;[1 1 1] Spawn un personnage aléatoire en fonction d'un temps aléatoire
  (`KismetSystemLibrary.Delay` (`KismetMathLibrary.RandomFloatInRange` 0.5 1.5))
  (if (`self.CanSpawn`)
    (bind _returnvalue (`AIBlueprintHelperLibrary.SpawnAIFromClass` "/Game/Blueprints/AI/Humans/HumanParent_BP.HumanParent_BP_C" "/Game/Blueprints/AI/Necessary/NPC_BT.NPC_BT" (`SceneComponent.K2_GetComponentLocation` (`self.BoxStart`))))
    (`self.MoveToActor` _returnvalue (`self.BoxEnd`))
    (`self.SpawnPeople`)))

(event `self.BoxEnd.OnComponentBeginOverlap`
  (params (OverlappedComponent :type "PrimitiveComponent Object Reference") (OtherActor :type "Actor Object Reference") (OtherComp :type "PrimitiveComponent Object Reference") (OtherBodyIndex :type Integer) (bFromSweep :type Boolean) (SweepResult :type "HitResult Structure (by ref)"))
  (bind _theplayer (`self.ThePlayer`))
  ;[1 1 1] Tend le passport quand il est proche du bureau
  (if (!= OtherActor (`self.TheHuman`))
    (bind _ashuman_parent_bp (cast `/Game/Blueprints/AI/Humans/HumanParent_BP` OtherActor))
    (bind _output_get (set `self.TheHuman` _ashuman_parent_bp))
    (`/Game/Essential/ThePlayerCamera.SpawnPaperHuman` _theplayer _output_get)
    (`/Game/Essential/ThePlayerCamera.SpawnHumanInfos` _theplayer (`/Game/Blueprints/AI/Humans/HumanParent_BP.Prenom` _output_get) (`/Game/Blueprints/AI/Humans/HumanParent_BP.TravelType` _output_get) (`/Game/Blueprints/AI/Humans/HumanParent_BP.Duration` _output_get))
    (`/Engine/EditorBlueprintResources/StandardMacros.DoOnce` false
      (:`Completed`
        (`/Game/Essential/ThePlayerCamera.BaisseJaugeHuman` (`self.ThePlayer`))))))

(event `self.BoxStart.OnComponentBeginOverlap`
  (params (OverlappedComponent :type "PrimitiveComponent Object Reference") (OtherActor :type "Actor Object Reference") (OtherComp :type "PrimitiveComponent Object Reference") (OtherBodyIndex :type Integer) (bFromSweep :type Boolean) (SweepResult :type "HitResult Structure (by ref)"))
  ;[1 1 1] Verifie que rien n'est en collision aveec la boite de spawn
  (set `self.CanSpawn` false))

(event `self.BoxForDestroy.OnComponentBeginOverlap`
  (params (OverlappedComponent :type "PrimitiveComponent Object Reference") (OtherActor :type "Actor Object Reference") (OtherComp :type "PrimitiveComponent Object Reference") (OtherBodyIndex :type Integer) (bFromSweep :type Boolean) (SweepResult :type "HitResult Structure (by ref)"))
  (`self.K2_DestroyActor` OtherActor))

(fn `MoveToActor`
  (params (`WhoNeedsToGo?` :type "Object Object Reference") (WhereToGo :type "SceneComponent Object Reference"))
  (bind _ashuman_parent_bp (cast `/Game/Blueprints/AI/Humans/HumanParent_BP` `WhoNeedsToGo?`))
  (bind _returnvalue (`AIBlueprintHelperLibrary.GetBlackboard` _ashuman_parent_bp))
  (`BlackboardComponent.SetValueAsVector` _returnvalue "LocationToGo" (`SceneComponent.K2_GetComponentLocation` WhereToGo))
  (`BlackboardComponent.SetValueAsBool` _returnvalue "CanMove" true))

(fn `No`
  (bind _thehuman (`self.TheHuman`))
  (bind _theplayer (`self.ThePlayer`))
  (bind _theplayer_2 (`self.ThePlayer`))
  (`/Engine/EditorBlueprintResources/StandardMacros.IsValid` _theplayer
    (:`Is Valid`
      (`/Game/Essential/ThePlayerCamera.ChangeJaugesHuman` _theplayer (`/Game/Blueprints/AI/Humans/HumanParent_BP.IsGoodGuy` _thehuman))
      (`/Game/Blueprints/Spring/Spring_Bp.Boing` (`self.MySpring`))
      (`Character.LaunchCharacter` _thehuman (0.0 0.0 1000.0) false false)
      (`/Game/Essential/ThePlayerCamera.DestroyPaperHuman` _theplayer_2)
      (`/Game/Essential/ThePlayerCamera.DestroyHumanDescription` _theplayer_2))))

(fn `UserConstructionScript`)

(fn `Yes`
  (bind _thehuman (`self.TheHuman`))
  (bind _theplayer (`self.ThePlayer`))
  (bind _theplayer_2 (`self.ThePlayer`))
  (`/Engine/EditorBlueprintResources/StandardMacros.IsValid` _theplayer
    (:`Is Valid`
      (`/Game/Essential/ThePlayerCamera.ChangeJaugesHuman` _theplayer (not (`/Game/Blueprints/AI/Humans/HumanParent_BP.IsGoodGuy` _thehuman)))
      (`self.MoveToActor` _thehuman (`self.BoxForDestroy`))
      (`/Game/Essential/ThePlayerCamera.DestroyPaperHuman` _theplayer_2)
      (`/Game/Essential/ThePlayerCamera.DestroyHumanDescription` _theplayer_2))))