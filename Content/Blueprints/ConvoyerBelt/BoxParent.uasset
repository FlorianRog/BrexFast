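; Parent conveyor-belt package for a customs-style inspection game, randomly sized, with a random sender (company or individual) and DataTable package type; pets get a crate mesh.
; BeginPlay enters a cascade of paper checks by current day, each calling earlier ones, so requirements accumulate.
; Applicable papers are rolled by percentage and ANDed into IsAGoodBox.
; Tick reddens the box as TimePackage drops; after touching the belt, it destroys overlapping boxes.
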(event `self.Boite.OnComponentBeginOverlap`
  (params (OverlappedComponent :type "PrimitiveComponent Object Reference") (OtherActor :type "Actor Object Reference") (OtherComp :type "PrimitiveComponent Object Reference") (OtherBodyIndex :type Integer) (bFromSweep :type Boolean) (SweepResult :type "HitResult Structure (by ref)"))
  (if (!= OtherActor self)
    (cast `/Game/Blueprints/ConvoyerBelt/ConvoyerBelt_BP` OtherActor
      (:`then`
        (set `self.CanDestroy` true))
      (:`CastFailed`
        (cast `/Game/Blueprints/ConvoyerBelt/BoxParent` OtherActor)
        (if (`self.CanDestroy`)
          (`self.K2_DestroyActor` OtherActor))))))

(event `self.ReceiveBeginPlay`
  (bind _thebox (`self.TheBox`))
  (bind _asthe_player_camera_bp (cast `/Game/Essential/ThePlayerCamera_BP` (`GameplayStatics.GetPlayerPawn` 0)))
  (set `self.ThePlayerCamera` _asthe_player_camera_bp)
  (bind _asmy_player_controller (cast `/Game/Essential/MyPlayerController` (`GameplayStatics.GetPlayerController` 0)))
  (set `self.ThePlayer` _asmy_player_controller)
  (if (`KismetMathLibrary.RandomBool`)
    (set `self.Entreprise?` true)
    (set `self.From` "Entreprise")
    (else
      (set `self.Particulier?` true)
      (set `self.From` "Particulier")))
  (bind _outrownames (`DataTableFunctionLibrary.GetDataTableRowNames` "/Game/Blueprints/Databases/Packages/BD_PackageType.BD_PackageType"))
  (set `self.RandomPackageType` (`KismetMathLibrary.RandomIntegerInRange` 0 (- (`KismetArrayLibrary.Array_Length` _outrownames) 1)))
  (for (_array_element _array_index) _outrownames
    (if (== _array_index (`self.RandomPackageType`))
      (bind _returnvalue (`|GetDataTableRow` "/Game/Blueprints/Databases/Packages/BD_PackageType.BD_PackageType" _array_element)
        (:`then`
          (bind (_packagetype _ispet _isdangerous _isstup _isother) (break `/Game/Blueprints/Databases/Packages/STDT_PackageType` _returnvalue))
          (set `self.PackageType` _packagetype)
          (set `self.IsAPet` _ispet)
          (set `self.IsDangerous` _isdangerous)
          (set `self.IsStup` _isstup)
          (set `self.IsOther` _isother)))))
  ;[1 1 1] Change the box
  (if (`self.IsAPet`)
    (`StaticMeshComponent.SetStaticMesh` _thebox "/Game/Assets/StaticMeshes/varisalacanelle.varisalacanelle")
    (`PrimitiveComponent.SetMaterial` _thebox 0 "/Game/Assets/MaterialAndTextures/Materiaux/BaseTexture/Childs/BT_CaisseTransport.BT_CaisseTransport")
    (`SceneComponent.SetWorldScale3D` _thebox (`KismetMathLibrary.MakeVector` (`KismetMathLibrary.RandomFloatInRange` 0.5 1.0) (`KismetMathLibrary.RandomFloatInRange` 0.5 1.0) (`KismetMathLibrary.RandomFloatInRange` 0.5 1.0))))
  (switch `int` (`/Game/Essential/MyPlayerController.CurrentDay` (`self.ThePlayer`))
    (:`Default`
      (`self.SetAutorisationDangerous` :!label _label))
    (:`1`
      (`self.CheckEtiquette` :!label _label_2))
    (:`2`
      (goto _label_2))
    (:`3`
      (`self.CheckAttestationAcquittement` :!label _label_3))
    (:`4`
      (goto _label_3))
    (:`5`
      (`self.CheckEntrepriseEORI` :!label _label_4))
    (:`6`
      (goto _label_4))
    (:`7`
      (`self.CheckPassePortPet` :!label _label_5))
    (:`8`
      (goto _label_5))
    (:`9`
      (`self.CheckDAE` :!label _label_6))
    (:`10`
      (goto _label_6))
    (:`11`
      (`self.CheckSpecialAutorisation` :!label _label_7))
    (:`12`
      (goto _label_7))
    (:`13`
      (`self.CheckCertificatEURMED` :!label _label_8))
    (:`14`
      (goto _label_8))
    (:`15`
      (`self.CheckVaccination` :!label _label_9))
    (:`16`
      (goto _label_9))
    (:`17`
      (`self.CheckCertificatMedical` :!label _label_10))
    (:`18`
      (goto _label_10))
    (:`19`
      (`self.CheckSPS` :!label _label_11))
    (:`20`
      (goto _label_11))
    (:`21`
      (goto _label))))

(event `SetGoodBox`
  ;[1 1 1] Directive change stat
  ;;[1 1 1] Set is a good box
  (for _array_element (`self.IsInGoodWay`)
    (set `self.IsAGoodBox` (and _array_element (`self.IsAGoodBox`)))))

(event `self.ReceiveTick`
  (params (DeltaSeconds :type "Float (single-precision)"))
  (`MeshComponent.SetScalarParameterValueOnMaterials` (`self.TheBox`) "LerpToTurnRed" (- 1.0 (/ (`/Game/Essential/ThePlayerCamera_BP.TimePackage` (`self.ThePlayerCamera`)) 100.0))))

(event `CheckEtiquette`
  ;[1 1 1] Directive change stat
  ;;[1 1 1] CheckEtiquette
  (bind _output_get (set `self.RandomFloatForChecks` (`KismetMathLibrary.RandomFloatInRange` 0.0 100.0)))
  (bind _output_get_2 (set `self.HaveEtiquette` (<= _output_get (`self.PercentToHaveEtiquette`))))
  (`KismetArrayLibrary.Array_Add` (`self.IsInGoodWay`) _output_get_2)
  (`self.SetGoodBox`))

(event `CheckAttestationAcquittement`
  ;[1 1 1] Directive change stat
  ;;[1 1 1] CheckAttestationAcquittement
  (bind _output_get (set `self.RandomFloatForChecks` (`KismetMathLibrary.RandomFloatInRange` 0.0 100.0)))
  (bind _output_get_2 (set `self.HaveAttestationAcquittement` (<= _output_get (`self.PercentToHaveAcquittement`))))
  (`KismetArrayLibrary.Array_Add` (`self.IsInGoodWay`) _output_get_2)
  (`self.CheckEtiquette`))

(event `CheckEntrepriseEORI`
  ;[1 1 1] Directive change stat
  ;;[1 1 1] CheckEORI
  (if (`self.Entreprise?`)
    (bind _output_get (set `self.RandomFloatForChecks` (`KismetMathLibrary.RandomFloatInRange` 0.0 100.0)))
    (bind _output_get_2 (set `self.HaveEORI` (<= _output_get (`self.PercentEORI`))))
    (`KismetArrayLibrary.Array_Add` (`self.IsInGoodWay`) _output_get_2)
    (`self.CheckAttestationAcquittement`)
    (else
      (`self.CheckAttestationAcquittement`))))

(event `CheckPassePortPet`
  ;[1 1 1] Directive change stat
  ;;[1 1 1] CheckPasseportAnimals
  (if (`self.IsAPet`)
    (bind _output_get (set `self.RandomFloatForChecks` (`KismetMathLibrary.RandomFloatInRange` 0.0 100.0)))
    (bind _output_get_2 (set `self.HavePasseportAnimal` (<= _output_get (`self.PercentPasseportAnimal`))))
    (`KismetArrayLibrary.Array_Add` (`self.IsInGoodWay`) _output_get_2)
    (`self.CheckEntrepriseEORI`)
    (else
      (`self.CheckEntrepriseEORI`))))

(event `CheckDAE`
  ;[1 1 1] Directive change stat
  ;;[1 1 1] CheckDAE
  (bind _output_get (set `self.RandomFloatForChecks` (`KismetMathLibrary.RandomFloatInRange` 0.0 100.0)))
  (bind _output_get_2 (set `self.HaveDAE` (<= _output_get (`self.PercentDAE`))))
  (`KismetArrayLibrary.Array_Add` (`self.IsInGoodWay`) _output_get_2)
  (`self.CheckPassePortPet`))

(event `CheckSpecialAutorisation`
  (bind _isstup (`self.IsStup`))
  ;[1 1 1] Directive change stat
  ;;[1 1 1] CheckSpecialAutorisation
  (if (select `bool` (`self.DangerousAutorisationPassed`) :`false` _isstup :`true` (and _isstup (`self.IsDangerous`)))
    (bind _output_get (set `self.RandomFloatForChecks` (`KismetMathLibrary.RandomFloatInRange` 0.0 100.0)))
    (bind _output_get_2 (set `self.HaveSpecialAutorisation` (<= _output_get (`self.PercentToHaveSpecialAutorisation`))))
    (`KismetArrayLibrary.Array_Add` (`self.IsInGoodWay`) _output_get_2)
    (`self.CheckDAE`)
    (else
      (`self.CheckDAE`))))

(event `CheckCertificatEURMED`
  ;[1 1 1] Directive change stat
  ;;[1 1 1] CheckCerticatEURMED
  (if (`self.Particulier?`)
    (bind _output_get (set `self.RandomFloatForChecks` (`KismetMathLibrary.RandomFloatInRange` 0.0 100.0)))
    (bind _output_get_2 (set `self.HaveEURMED` (<= _output_get (`self.PercentToHaveCertificatEURMED`))))
    (`KismetArrayLibrary.Array_Add` (`self.IsInGoodWay`) _output_get_2)
    (`self.CheckSpecialAutorisation`)
    (else
      (`self.CheckSpecialAutorisation`))))

(event `CheckVaccination`
  ;[1 1 1] Directive change stat
  ;;[1 1 1] CheckVaccination
  (if (`self.IsAPet`)
    (bind _output_get (set `self.RandomFloatForChecks` (`KismetMathLibrary.RandomFloatInRange` 0.0 100.0)))
    (bind _output_get_2 (set `self.HaveVaccination` (<= _output_get (`self.PercentToHaveVaccination`))))
    (`KismetArrayLibrary.Array_Add` (`self.IsInGoodWay`) _output_get_2)
    (`self.CheckCertificatEURMED`)
    (else
      (`self.CheckCertificatEURMED`))))

(event `CheckCertificatMedical`
  ;[1 1 1] Directive change stat
  ;;[1 1 1] CheckCertificatMedical
  (if (`self.IsAPet`)
    (bind _output_get (set `self.RandomFloatForChecks` (`KismetMathLibrary.RandomFloatInRange` 0.0 100.0)))
    (bind _output_get_2 (set `self.HaveCertifMedical` (<= _output_get (`self.PercentToHaveCertificatMedical`))))
    (`KismetArrayLibrary.Array_Add` (`self.IsInGoodWay`) _output_get_2)
    (`self.CheckVaccination`)
    (else
      (`self.CheckVaccination`))))

(event `CheckSPS`
  ;[1 1 1] Directive change stat
  ;;[1 1 1] CheckSPS
  (if (`self.IsAPet`)
    (bind _output_get (set `self.RandomFloatForChecks` (`KismetMathLibrary.RandomFloatInRange` 0.0 100.0)))
    (bind _output_get_2 (set `self.HaveSPS` (<= _output_get (`self.PercentToHaveSPS`))))
    (`KismetArrayLibrary.Array_Add` (`self.IsInGoodWay`) _output_get_2)
    (`self.CheckCertificatMedical`)
    (else
      (`self.CheckCertificatMedical`))))

(event `SetAutorisationDangerous`
  ;[1 1 1] Directive change stat
  ;;[1 1 1] SetAutorisationDangerous
  (set `self.DangerousAutorisationPassed` true)
  (`self.CheckSPS`))

(fn `GetPapers`
  (returns (HaveEtiquette :type Boolean) (HaveAttestationAcquittement :type Boolean) (HaveEORI :type Boolean) (HavePasseportAnimal :type Boolean) (HaveDAE :type Boolean) (HaveSpecialAutorisation :type Boolean) (HaveEURMED :type Boolean) (HaveVaccination :type Boolean) (HaveCertifMedical :type Boolean) (HaveSPS :type Boolean))
  (return (`self.HaveEtiquette`) (`self.HaveAttestationAcquittement`) (`self.HaveEORI`) (`self.HavePasseportAnimal`) (`self.HaveDAE`) (`self.HaveSpecialAutorisation`) (`self.HaveEURMED`) (`self.HaveVaccination`) (`self.HaveCertifMedical`) (`self.HaveSPS`)))

(fn `UserConstructionScript`
  (bind _boite (`self.Boite`))
  (bind _minscale (`self.MinScale`))
  (bind _maxscale (`self.MaxScale`))
  (`self.SetActorScale3D` (`KismetMathLibrary.MakeVector` (`KismetMathLibrary.RandomFloatInRange` _minscale _maxscale) (`KismetMathLibrary.RandomFloatInRange` _minscale _maxscale) (`KismetMathLibrary.RandomFloatInRange` _minscale _maxscale)))
  (`SceneComponent.SetRelativeScale3D` _boite (* (`SceneComponent.RelativeScale3D` _boite) 1.6)))