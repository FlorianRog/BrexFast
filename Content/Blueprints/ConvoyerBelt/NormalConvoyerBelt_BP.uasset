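; Conveyor belt actor that carries BoxParent actors along its length and removes them at a destruction zone.
; Each tick, it offsets every box overlapping NormalMovementBox along NormalDirection's forward vector, scaled by Speed and delta time.
; Movement is a direct world offset without sweep, so it ignores collision along the way.
; Any BoxParent that begins overlapping DestructionBox is destroyed.
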(event `self.ReceiveTick`
  (params (DeltaSeconds :type "Float (single-precision)"))
  ;[1 1 1] Adding movement to the convoyer belt
  (for _array_element (`PrimitiveComponent.GetOverlappingActors` (`self.NormalMovementBox`) "/Game/Blueprints/ConvoyerBelt/Boxes/BoxParent.BoxParent_C")
    (if (!= _array_element self)
      (`self.K2_AddActorWorldOffset` _array_element (* (`SceneComponent.GetForwardVector` (`self.NormalDirection`)) (* DeltaSeconds (`self.Speed`))) false false))))

(event `self.DestructionBox.OnComponentBeginOverlap`
  (params (OverlappedComponent :type "PrimitiveComponent Object Reference") (OtherActor :type "Actor Object Reference") (OtherComp :type "PrimitiveComponent Object Reference") (OtherBodyIndex :type Integer) (bFromSweep :type Boolean) (SweepResult :type "HitResult Structure (by ref)"))
  (cast `/Game/Blueprints/ConvoyerBelt/Boxes/BoxParent` OtherActor)
  (`self.K2_DestroyActor` OtherActor))

(fn `UserConstructionScript`)