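; Visa document actor whose appearance reflects its traveler type: work, study or travel.
; The construction script switches on TravelerType to give the Passeport component a type-specific material and update its text renders.
; Work and travel display the enum name as the second text, while study overrides both texts with French literals.
; The event graph holds only disabled stubs, so there is no runtime logic.
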(fn `UserConstructionScript`
  (bind _passeport (`self.Passeport`))
  (bind _travelertype (`self.TravelerType`))
  (switch `string` _travelertype
    (:`Travail`
      (`PrimitiveComponent.SetMaterial` _passeport 0 "/Game/Assets/MaterialAndTextures/Materiaux/BaseColor/Childs/inst_cc8e35.inst_cc8e35")
      (`TextRenderComponent.K2_SetText` (`self.TextRender1`) (`KismetTextLibrary.Conv_StringToText` _travelertype) :!label _label))
    (:`Etudes`
      (`PrimitiveComponent.SetMaterial` _passeport 0 "/Game/Assets/MaterialAndTextures/Materiaux/BaseColor/Childs/inst_40407a.inst_40407a")
      (`TextRenderComponent.K2_SetText` (`self.TextRender`) "Visa")
      (`TextRenderComponent.K2_SetText` (`self.TextRender1`) "d'étude"))
    (:`Voyage`
      (`PrimitiveComponent.SetMaterial` _passeport 0 "/Game/Assets/MaterialAndTextures/Materiaux/BaseColor/Childs/inst_b33939.inst_b33939")
      (goto _label))))